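; BP_HUD_Menu is the HUD for the main menu, setting up its input and widgets on BeginPlay.
; It switches the owning player to UI-only input with a visible cursor, creates the FPS widget, then creates and displays the menu widget.
; The FPS widget is stored but hidden until ShowFPS adds it at a high Z-order, and HideFPS removes it.
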(event Custom|Hide%20FPS
  (Widget|RemovefromParent (Variables|Default|GetWidgetFPS)))

(event Custom|Set%20Input%20Settings
  (bind _returnvalue (Game|Player|GetOwningPlayerController))
  (Input|SetInputModeUIOnly _returnvalue 0 "DoNotLock")
  (Variables|/Script/Engine.PlayerController|SetbShowMouseCursor _returnvalue true))

(event Custom|CreateWidgetMenu
  (bind _returnvalue (UserInterface|CreateWidget "/Game/-Blueprints/-Menu/Widgets/WB_Menu.WB_Menu_C" (Game|Player|GetOwningPlayerController)))
  (UserInterface|Viewport|AddtoViewport _returnvalue 0))

(event Custom|CreateWidgetFPS
  (bind _returnvalue (UserInterface|CreateWidget "/Game/-Blueprints/-General/Widgets/WB_FPS.WB_FPS_C" (Game|Player|GetOwningPlayerController)))
  (Variables|Default|SetWidgetFPS _returnvalue))

(event Custom|Show%20FPS
  (UserInterface|Viewport|AddtoViewport (Variables|Default|GetWidgetFPS) 100))

(event EventBeginPlay
  (Utilities|FlowControl|Sequence
    (:then_0
      (CallFunction|SetInputSettings))
    (:then_1
      (CallFunction|CreateWidgetFPS))
    (:then_2
      (CallFunction|CreateWidgetMenu))))

(fn ConstructionScript)