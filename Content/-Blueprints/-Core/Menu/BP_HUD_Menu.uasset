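; Main menu HUD that puts the menu widget on screen and controls an optional FPS counter.
; On BeginPlay it creates WB_Menu, switches input to UI only and shows the mouse cursor.
; It also creates WB_FPS and displays it if the ShowFPS flag in the "info" save slot is set.
; ShowFPS and HideFPS events reuse that widget to add or remove the counter at runtime.
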(event Custom|Show%20FPS
  (UserInterface|Viewport|AddtoViewport (stale EventBeginPlay _returnvalue_3) 0))

(event Custom|Hide%20FPS
  (Widget|RemovefromParent (stale EventBeginPlay _returnvalue_3)))

(event EventBeginPlay
  (bind _returnvalue (Game|Player|GetOwningPlayerController))
  (Utilities|FlowControl|Sequence
    (:then_0
      (bind _returnvalue_2 (UserInterface|CreateWidget "/Game/-Blueprints/Widgets/Menu/WB_Menu.WB_Menu_C" _returnvalue))
      (UserInterface|Viewport|AddtoViewport _returnvalue_2 0)
      (Input|SetInputModeUIOnly _returnvalue _returnvalue_2 "DoNotLock")
      (Variables|/Script/Engine.PlayerController|SetbShowMouseCursor _returnvalue true))
    (:then_1
      (bind _returnvalue_3 (UserInterface|CreateWidget "/Game/-Blueprints/Widgets/WB_FPS.WB_FPS_C" (Game|Player|GetOwningPlayerController)))
      (bind _returnvalue_4 (SaveGame|LoadGamefromSlot "info"))
      (bind _asbp_save_game (Utilities|Casting|CastToBP_SaveGame _returnvalue_4))
      (if (Variables|/Game/-Blueprints/-Core/Save/BP_SaveGame.BP_SaveGame_C|GetShowFPS _asbp_save_game)
        (UserInterface|Viewport|AddtoViewport _returnvalue_3 0)
        (else
          (Widget|RemovefromParent _returnvalue_3))))))

(fn ConstructionScript)