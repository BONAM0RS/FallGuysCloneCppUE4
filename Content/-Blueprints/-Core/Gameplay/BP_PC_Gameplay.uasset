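; Gameplay player controller that handles player-info board, chat and exit-to-menu input, plus the character's gender.
; On possess with authority, it reads the saved sex from the "info" slot and applies it to the pawn through ServerChangeSex.
; The chat toggle switches cursor, input mode and pawn input, while separate events relay messages to the GameState or GameMode.
; The menu key destroys the session and opens L_Menu whether that succeeds or fails.
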(event Custom|SendChatMessageToGameState
  (params (Sender :type String) (Message :type String) (MessageType :type Byte))
  (bind _asbp_gs_gameplay (Utilities|Casting|CastToBP_GS_Gameplay (Game|GetGameState)))
  (Default|CallonChatMessageSendtoGameState _asbp_gs_gameplay Sender Message MessageType))

(event Custom|Local%20Change%20Sex
  (bind _returnvalue (SaveGame|LoadGamefromSlot "info"))
  (bind _asbp_save_game (Utilities|Casting|CastToBP_SaveGame _returnvalue))
  (CallFunction|ServerChangeSex (Variables|/Game/-Blueprints/-Core/Save/BP_SaveGame.BP_SaveGame_C|GetPlayerSex _asbp_save_game)))

(event Custom|Server%20Change%20Sex
  (params (Gender :type Boolean))
  (bind _asbp_char_gameplay (Utilities|Casting|CastToBP_Char_Gameplay (Pawn|GetControlledPawn)))
  (Variables|/Game/-Blueprints/-Core/Gameplay/BP_Char_Gameplay.BP_Char_Gameplay_C|SetGender _asbp_char_gameplay Gender))

(event Custom|Set%20Mesh
  (params (Gender :type Boolean))
  (CallFunction|ServerChangeSex Gender))

(event Custom|HideChat
  (Default|HideChat (Variables|/Game/-Blueprints/Widgets/Gameplay/Chat/WB_ChatOnScreen.WB_ChatOnScreen_C|GetWB_ChatBox (Variables|/Game/-Blueprints/-Core/Gameplay/BP_HUD_Gameplay.BP_HUD_Gameplay_C|GetWB_ChatOnScreen (Variables|Default|GetHUD%20Gameplay))))
  (Variables|Default|SetbShowMouseCursor false)
  (Input|SetInputModeGameOnly self)
  (Input|EnableInput (Pawn|GetControlledPawn) self))

(event Custom|CallOnChatMessageSendToGameMode
  (params (Sender :type String) (Message :type String) (MessageType :type Byte))
  ;[1 1 1] From GameMode
  (Default|CallOnChatMessageSendtoGameMode Sender Message MessageType))

(event Custom|SendChatMessageToGameMode
  (params (Sender :type String) (Message :type String) (MessageType :type Byte))
  (bind _asbp_gm_gameplay (Utilities|Casting|CastToBP_GM_Gameplay (Game|GetGameMode)))
  (Default|SendChatMessagetoAllPlayerControllers _asbp_gm_gameplay Sender Message MessageType))

(event EventPossess
  (params (PossessedPawn :type Pawn%20Object%20Reference))
  (Networking|SwitchHasAuthority
    (:Authority
      (CallFunction|LocalChangeSex))))

(event EventBeginPlay
  (bind _asbp_hud_gameplay (Utilities|Casting|CastToBP_HUD_Gameplay (HUD|GetHUD)))
  (Variables|Default|SetHUD%20Gameplay _asbp_hud_gameplay))

(event Input|ActionEvents|InputActionOpenPlayerInfoBorad
  (params (Key :type Key%20Structure :default "None"))
  (bind _hud_gameplay (Variables|Default|GetHUD%20Gameplay))
  (:Pressed
    (Default|ShowPlayersInfoBorad _hud_gameplay))
  (:Released
    (Default|HidePlayersInfoBoard _hud_gameplay)))

(event Input|ActionEvents|InputActionOpenChat
  (params (Key :type Key%20Structure :default "None"))
  (bind _returnvalue (Pawn|GetControlledPawn))
  (bind _self self)
  (bind _self_2 self)
  (bind _hud_gameplay (Variables|Default|GetHUD%20Gameplay))
  (bind _wb_chatonscreen (Variables|/Game/-Blueprints/-Core/Gameplay/BP_HUD_Gameplay.BP_HUD_Gameplay_C|GetWB_ChatOnScreen _hud_gameplay))
  (bind _wb_chatbox (Variables|/Game/-Blueprints/Widgets/Gameplay/Chat/WB_ChatOnScreen.WB_ChatOnScreen_C|GetWB_ChatBox _wb_chatonscreen))
  (:Pressed
    (if (== (Class|WidgetSwitcher|GetActiveWidgetIndex (Variables|/Game/-Blueprints/Widgets/Gameplay/Chat/WB_ChatBox.WB_ChatBox_C|GetWidgetSwitcher_0 (Variables|/Game/-Blueprints/Widgets/Gameplay/Chat/WB_ChatOnScreen.WB_ChatOnScreen_C|GetWB_ChatBox _wb_chatonscreen))) 0)
      (Default|ShowChat _wb_chatbox)
      (Variables|Default|SetbShowMouseCursor true)
      (Input|SetInputModeGameandUI _self (Variables|/Game/-Blueprints/Widgets/Gameplay/Chat/WB_ChatBox.WB_ChatBox_C|GetEditableTextBox_Message _wb_chatbox) "DoNotLock" true)
      (Input|DisableInput _returnvalue _self_2)
      (else
        (Default|HideChat _wb_chatbox)
        (Variables|Default|SetbShowMouseCursor false)
        (Input|SetInputModeGameOnly _self)
        (Input|EnableInput _returnvalue _self_2)))))

(event Input|ActionEvents|InputActionOpenMenu
  (params (Key :type Key%20Structure :default "None"))
  ;[1 1 1] Dont need if hide chat on clear in WB_ChatBox
)

(event Input|ActionEvents|InputActionOpenMenu
  (params (Key :type Key%20Structure :default "None"))
  (:Pressed
    (|DestroySession self
      (:OnSuccess
        _)
      (:OnFailure
        _))
    (Game|OpenLevel(byObjectReference) "/Game/Maps/Menu/L_Menu.L_Menu")))

(event Input|ActionEvents|InputActionOpenMenu
  (params (Key :type Key%20Structure :default "None"))
  ;[1 1 1] Tested Main Menu In Gameplay
)

(fn ConstructionScript)