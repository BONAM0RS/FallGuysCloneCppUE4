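; Gameplay game mode that relays chat messages to players and announces when someone leaves the server.
; SendChatMessageToAllPlayerControllers loops the GameState PlayerArray and passes sender, text and message type to each owning BP_PC_Gameplay.
; OnLogout reads the leaving player's name from BP_PS_Gameplay and broadcasts a disconnect notice through that same event.
; BeginPlay, Tick and PostLogin are empty.
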(event Custom|SendChatMessageToAllPlayerControllers
  (params (Sender :type String) (Message :type String) (MessageType :type Byte))
  (for _array_element (Variables|/Script/Engine.GameStateBase|GetPlayerArray (Game|GetGameState))
    (bind _asbp_pc_gameplay (Utilities|Casting|CastToBP_PC_Gameplay (Components|GetOwner _array_element)))
    (Default|CallonChatMessageSendtoGameMode _asbp_pc_gameplay Sender Message MessageType)))

(event EventBeginPlay)

(event EventTick
  (params (DeltaSeconds :type Float%20%28single-precision%29)))

(event EventPostLogin
  (params (NewPlayer :type Player%20Controller%20Object%20Reference)))

(event EventOnLogout
  (params (ExitingController :type Controller%20Object%20Reference))
  (bind _asbp_ps_gameplay (Utilities|Casting|CastToBP_PS_Gameplay (Variables|/Script/Engine.Controller|GetPlayerState ExitingController)))
  (CallFunction|SendChatMessagetoAllPlayerControllers (Utilities|String|ToString(Text) (Variables|/Game/-Blueprints/-Core/Gameplay/BP_PS_Gameplay.BP_PS_Gameplay_C|GetName _asbp_ps_gameplay)) " disconnecter from server" 2))

(fn ConstructionScript)