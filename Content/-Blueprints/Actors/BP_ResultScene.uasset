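; BP_ResultScene is a base actor for the results scene that players' cameras switch to when the result board is shown.
; It starts hidden, and the server caches the gameplay GameMode and GameState, then calls a virtual BindEvents hook.
; OnShowResultBoard reveals the scene through EnableVisibilityMulticast, calls a virtual PlacePlayers hook, then sets each player controller's view target to this actor.
; Both hooks are empty here, leaving event binding and player placement to child classes.
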(event Custom|Bind%20Events)

(event Custom|On%20Show%20Result%20Board
  (CallFunction|EnableVisibilityMulticast)
  (CallFunction|PlacePlayers)
  (CallFunction|SwitchPlayersCameratoResulsBoard))

(event Custom|Place%20Players)

(event Custom|Switch%20Players%20Camera%20To%20Resuls%20Board
  (for _array_element (Variables|/Script/Engine.GameStateBase|GetPlayerArray (Game|GetGameState))
    (bind _asbp_pc_gameplay (Utilities|Casting|CastToBP_PC_Gameplay (Components|GetOwner _array_element)))
    (Game|Player|SetViewTargetwithBlend _asbp_pc_gameplay self 0.0 "VTBlend_Linear" 0.0 false)))

(event Custom|Init%20Framework%20Actors
  (bind _asbp_gm_gameplay (Utilities|Casting|CastToBP_GM_Gameplay (Game|GetGameMode))
    (:then
      (bind _output_get (Variables|FrameworkActors|SetAs%20BP%20GM%20Gameplay%20Server _asbp_gm_gameplay))
      (Variables|FrameworkActors|SetAs%20BP%20GS%20Gameplay%20Server (Variables|/Game/-Blueprints/-Gameplay/Core/BP_GM_Gameplay.BP_GM_Gameplay_C|GetAs%20BP%20GS%20Gameplay%20Server _output_get)))
    (:CastFailed
      (CallFunction|PrintCastFailed self "BP_GM_Gameplay" true true))))

(event Custom|Enable%20Visibility%20Multicast
  (Rendering|SetVisibility (Variables|Default|GetDefaultSceneRoot) true true))

(event EventBeginPlay
  (Rendering|SetVisibility (Variables|Default|GetDefaultSceneRoot) false true)
  (if (Networking|IsServer)
    (CallFunction|InitFrameworkActors)
    (CallFunction|BindEvents)))

(fn ConstructionScript)