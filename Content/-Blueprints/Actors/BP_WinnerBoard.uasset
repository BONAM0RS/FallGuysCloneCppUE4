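; End-of-match winner board actor that stays hidden until it presents the winner to all players.
; ShowWinnerResultBoard reveals it, hides round-over popups, and moves players in a specific player state to the arrow slot through a teleport event named as multicast.
; It then switches every player's view to itself, shows their winner widget, and has the server-cached game state start the return-to-menu timer.
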(event Custom|Show%20Winner%20Result%20Board
  (CallFunction|EnableVisibility)
  (CallFunction|HideWidgetsandPlaceWinner)
  (CallFunction|SwitchPlayersCameratoWinnerBoard)
  (Default|CreateTimertoSendAllPlayerstoMenu (Variables|Default|GetAs%20BP%20GS%20Gameplay%20Server)))

(event Custom|Enable%20Visibility
  (Rendering|SetVisibility (Variables|Default|GetSceneComponent) true true)
  (Development|PrintString "ENABLE VISIBILITY" true true "(R=0.000000,G=0.660000,B=1.000000,A=1.000000)" 3.6e+02))

(event Custom|Teleport%20Player%20Multicast
  (params (Pawn%20Actor :type Actor%20Object%20Reference) (NewLocation :type Vector) (NewRotation :type Rotator))
  (Transformation|SetActorLocationAndRotation Pawn%20Actor NewLocation NewRotation false true))

(event Custom|Hide%20Widgets%20And%20Place%20Winner
  (bind _arrowplayerslot (Variables|Default|GetArrowPlayerSlot))
  (for _array_element (Variables|/Script/Engine.GameStateBase|GetPlayerArray (Game|GetGameState))
    (bind _asbp_pc_gameplay (Utilities|Casting|CastToBP_PC_Gameplay (Components|GetOwner _array_element)))
    (Default|HideRoundOverPopUpWidget _asbp_pc_gameplay)
    (bind _asbp_ps_gameplay (Utilities|Casting|CastToBP_PS_Gameplay _array_element))
    (if (Utilities|Enum|Equal(Enum) (Variables|/Game/-Blueprints/-Gameplay/Core/BP_PS_Gameplay.BP_PS_Gameplay_C|GetPlayerState _asbp_ps_gameplay) (Utilities|Enum|LiteralenumEnum_PlayerStates "NewEnumerator1"))
      (bind _asbp_char_gameplay (Utilities|Casting|CastToBP_Char_Gameplay (Variables|/Script/Engine.PlayerState|GetPawnPrivate _array_element)))
      (Default|EnableVisibilityandCollisionMulticast _asbp_char_gameplay)
      (CallFunction|TeleportPlayerMulticast (Variables|/Script/Engine.PlayerState|GetPawnPrivate _array_element) (Transformation|GetWorldLocation _arrowplayerslot) (Transformation|GetWorldRotation _arrowplayerslot)))))

(event Custom|Switch%20Players%20Camera%20To%20Winner%20Board
  (for _array_element (Variables|/Script/Engine.GameStateBase|GetPlayerArray (Game|GetGameState))
    (bind _asbp_pc_gameplay (Utilities|Casting|CastToBP_PC_Gameplay (Components|GetOwner _array_element)))
    (Game|Player|SetViewTargetwithBlend _asbp_pc_gameplay self 0.0 "VTBlend_Linear" 0.0 false)
    (Default|ShowWinnerBoardWidget _asbp_pc_gameplay)))

(event EventBeginPlay
  (Rendering|SetVisibility (Variables|Default|GetSceneComponent) false true)
  (if (Networking|IsServer)
    (bind _asbp_gs_gameplay (Utilities|Casting|CastToBP_GS_Gameplay (Game|GetGameState)))
    (Variables|Default|SetAs%20BP%20GS%20Gameplay%20Server _asbp_gs_gameplay)))

(fn ConstructionScript)