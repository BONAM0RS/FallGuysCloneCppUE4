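; BP_EliminationTrigger is a trigger actor that signals player elimination when an actor begins overlapping it.
; On the server, BeginPlay registers the trigger with the gameplay game state as its elimination trigger.
; The overlap handler runs the parent trigger logic, then broadcasts the OnPlayerEliminated dispatcher without checking the overlapping actor itself.
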(event EventBeginPlay
  (|CallParentFunction)
  (if (Networking|IsServer)
    (Variables|/Game/-Blueprints/-Gameplay/Core/BP_GS_Gameplay.BP_GS_Gameplay_C|SetBP%20Elimination%20Trigger (Variables|Default|GetAs%20BP%20GS%20Gameplay) self)))

(fn ConstructionScript
  (|CallParentFunction))

(fn OnTriggerActorBeginOverlap
  (params (Overlapped%20Actor :type Actor%20Object%20Reference))
  (|CallParentFunction Overlapped%20Actor)
  (Default|CallOnPlayerEliminated))