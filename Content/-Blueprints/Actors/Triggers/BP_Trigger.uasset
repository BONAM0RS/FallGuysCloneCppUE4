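; BP_Trigger is a trigger actor with a box component that reacts to overlaps only during one specific round state.
; It caches BP_GS_Gameplay on BeginPlay, and CanOverlap checks that it runs on the server and that the round state matches.
; Accepted actor overlaps are passed to OnTriggerActorBeginOverlap, which is empty here, so the asset appears to serve as a base for specific triggers.
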(event OnComponentBeginOverlap(Box)
  (params (OverlappedComponent :type Primitive%20Component%20Object%20Reference) (OtherActor :type Actor%20Object%20Reference) (OtherComp :type Primitive%20Component%20Object%20Reference) (OtherBodyIndex :type Integer) (bFromSweep :type Boolean) (SweepResult :type Hit%20Result%20Structure%20%28by%20ref%29)))

(event EventBeginPlay
  (bind _asbp_gs_gameplay (Utilities|Casting|CastToBP_GS_Gameplay (Game|GetGameState))
    (:then
      (Variables|Default|SetAs%20BP%20GS%20Gameplay _asbp_gs_gameplay))
    (:CastFailed
      (CallFunction|PrintCastFailed self _asbp_gs_gameplay true true))))

(event Collision|EventActorBeginOverlap
  (params (OtherActor :type Actor%20Object%20Reference))
  (bind _can_overlap (CallFunction|CanOverlap OtherActor))
  (if _can_overlap
    (CallFunction|OnTriggerActorBeginOverlap OtherActor)))

(fn ConstructionScript)

(fn CanOverlap
  (params (Other%20Actor :type Actor%20Object%20Reference))
  (if (Networking|IsServer)
    (if (Utilities|Enum|Equal(Enum) (Variables|/Game/-Blueprints/-Gameplay/Core/BP_GS_Gameplay.BP_GS_Gameplay_C|GetRound%20State (Variables|Default|GetAs%20BP%20GS%20Gameplay)) (Utilities|Enum|LiteralenumEnum_RoundStates "NewEnumerator1"))
      (return true)
      (else
        (return false)))))

(fn OnTriggerActorBeginOverlap
  (params (Overlapped%20Actor :type Actor%20Object%20Reference)))