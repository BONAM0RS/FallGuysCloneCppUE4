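; BP_PlayerTrigger is a trigger actor that only accepts overlaps from player characters.
; It overrides Can Overlap, running the parent check first and then Is Player.
; Is Player requires a BP_Char_Gameplay with a BP_PS_Gameplay player state, and caches both as the last overlapped character and player state when the check passes.
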(fn ConstructionScript)

(fn CanOverlap
  (params (Other%20Actor :type Actor%20Object%20Reference))
  (bind _can_overlap (|CallParentFunction Other%20Actor))
  (if _can_overlap
    (bind _is_player (CallFunction|IsPlayer Other%20Actor))
    (return _is_player)
    (else
      (return false))))

(fn IsPlayer
  (params (Actor :type Actor%20Object%20Reference))
  (bind _asbp_char_gameplay (Utilities|Casting|CastToBP_Char_Gameplay Actor))
  (bind _asbp_ps_gameplay (Utilities|Casting|CastToBP_PS_Gameplay (Variables|/Script/Engine.Pawn|GetPlayerState _asbp_char_gameplay)))
  (if (and (Utilities|IsValid _asbp_ps_gameplay) (Utilities|IsValid _asbp_char_gameplay))
    (Variables|Default|SetLast%20Overlapped%20BP%20Char%20Gameplay _asbp_char_gameplay)
    (Variables|Default|SetLast%20Overlapped%20BP%20PS%20Gameplay _asbp_ps_gameplay)
    (return true)
    (else
      (return false))))