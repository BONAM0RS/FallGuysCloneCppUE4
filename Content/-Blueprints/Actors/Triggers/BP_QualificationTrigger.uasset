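; Trigger actor that marks a player as qualified on entering it, such as at a finish or goal.
; It extends a parent trigger's overlap check to reject players whose gameplay PlayerState is already in the state this trigger assigns.
; On a valid overlap it runs the parent logic, sets that state on the last overlapped player state and fires OnPlayerQualified.
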(fn ConstructionScript
  (|CallParentFunction))

(fn CanOverlap
  (params (Other%20Actor :type Actor%20Object%20Reference))
  (bind _can_overlap (|CallParentFunction Other%20Actor))
  (if _can_overlap
    (if (!= (Variables|/Game/-Blueprints/-Gameplay/Core/BP_PS_Gameplay.BP_PS_Gameplay_C|GetPlayerState (Variables|Default|GetLast%20Overlapped%20BP%20PS%20Gameplay)) (Utilities|Enum|LiteralenumEnum_PlayerStates "NewEnumerator1"))
      (return true)
      (else
        (return false)))
    (else
      (return false))))

(fn OnTriggerActorBeginOverlap
  (params (Overlapped%20Actor :type Actor%20Object%20Reference))
  (|CallParentFunction Overlapped%20Actor)
  (Default|SetState (Variables|Default|GetLast%20Overlapped%20BP%20PS%20Gameplay) "NewEnumerator1")
  (Default|CallOnPlayerQualified0))