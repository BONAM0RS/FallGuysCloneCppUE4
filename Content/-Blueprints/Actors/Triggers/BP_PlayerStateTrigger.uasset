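; BP_PlayerStateTrigger is a trigger actor that marks overlapping players as qualified or eliminated.
; On BeginPlay it takes its trigger type from the current level's data row.
; It extends the parent overlap check to accept only players in the default state while the game state's player-state score differs from its maximum.
; On overlap it sets the player state accordingly and calls the matching qualified or eliminated event.
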(event EventBeginPlay
  (|CallParentFunction)
  (bind _player_state_trigger_type (CallFunction|GetCurrentLevelInfoRowData))
  (Variables|Default|SetPlayer%20State%20Trigger%20Type _player_state_trigger_type))

(fn ConstructionScript)

(fn CanOverlap
  (params (Other%20Actor :type Actor%20Object%20Reference))
  (bind _as_bp_gs_gameplay (Variables|Default|GetAs%20BP%20GS%20Gameplay))
  (bind _can_overlap (|CallParentFunction Other%20Actor))
  (if _can_overlap
    (if (and (Utilities|Enum|Equal(Enum) (Variables|/Game/-Blueprints/-Gameplay/Core/BP_PS_Gameplay.BP_PS_Gameplay_C|GetPlayerState (Variables|Default|GetLast%20Overlapped%20BP%20PS%20Gameplay)) (Utilities|Enum|LiteralenumEnum_PlayerStates "NewEnumerator0")) (!= (Variables|/Game/-Blueprints/-Gameplay/Core/BP_GS_Gameplay.BP_GS_Gameplay_C|GetCurrent%20Player%20States%20Score _as_bp_gs_gameplay) (Variables|/Game/-Blueprints/-Gameplay/Core/BP_GS_Gameplay.BP_GS_Gameplay_C|GetMax%20Player%20States%20Score _as_bp_gs_gameplay)))
      (return true)
      (else
        (return false)))
    (else
      (return false))))

(fn OnTriggerActorBeginOverlap
  (params (Overlapped%20Actor :type Actor%20Object%20Reference))
  (bind _last_overlapped_bp_ps_gameplay (Variables|Default|GetLast%20Overlapped%20BP%20PS%20Gameplay))
  (|CallParentFunction Overlapped%20Actor)
  (switch Utilities|FlowControl|Switch|SwitchonEnum_LevelPlayerStateTriggerTypes (Variables|Default|GetPlayer%20State%20Trigger%20Type)
    (:NewEnumerator0
      (Default|SetState _last_overlapped_bp_ps_gameplay "NewEnumerator1")
      (Default|CallOnPlayerQualified))
    (:NewEnumerator1
      (Default|SetState _last_overlapped_bp_ps_gameplay "NewEnumerator4")
      (Default|CallOnPlayerEliminated))))