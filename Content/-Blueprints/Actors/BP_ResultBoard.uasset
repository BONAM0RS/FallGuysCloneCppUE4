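; Base result board actor that stays hidden until the game state calls for its board type, then becomes the players' end-screen view.
; The server caches BP_GS_Gameplay, and BindEvents hooks its show-result-board dispatcher.
; On a type match it multicasts visibility, calls PlacePlayers and blends every player controller's view to itself.
; PlacePlayers is an empty hook, with a multicast teleport helper available for positioning pawns.
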(event Custom|On%20Show%20Result%20Board
  (if (Utilities|Enum|Equal(Enum) (Variables|/Game/-Blueprints/-Gameplay/Core/BP_GS_Gameplay.BP_GS_Gameplay_C|GetSelected%20Result%20Board%20Type (Variables|FrameworkActors|GetAs%20BP%20GS%20Gameplay%20Server)) (Variables|Default|GetResult%20Board%20Type))
    (CallFunction|EnableVisibilityMulticast)
    (CallFunction|PlacePlayers)
    (CallFunction|SwitchPlayersCameratoResulsBoard)))

(event Custom|Teleport%20Player%20Multicast
  (params (Pawn%20Actor :type Actor%20Object%20Reference) (NewLocation :type Vector) (NewRotation :type Rotator))
  (Transformation|SetActorLocationAndRotation Pawn%20Actor NewLocation NewRotation false true))

(event Custom|Place%20Players)

(event Custom|Switch%20Players%20Camera%20To%20Resuls%20Board
  (for _array_element (Variables|/Script/Engine.GameStateBase|GetPlayerArray (Game|GetGameState))
    (bind _asbp_pc_gameplay (Utilities|Casting|CastToBP_PC_Gameplay (Components|GetOwner _array_element)))
    (Game|Player|SetViewTargetwithBlend _asbp_pc_gameplay self 0.0 "VTBlend_Linear" 0.0 false)))

(event Custom|Init%20Framework%20Actors
  (bind _asbp_gs_gameplay (Utilities|Casting|CastToBP_GS_Gameplay (Game|GetGameState)))
  (Variables|FrameworkActors|SetAs%20BP%20GS%20Gameplay%20Server _asbp_gs_gameplay))

(event Custom|Bind%20Events
  (EventDispatchers|BindEventtoOnShowResultBoardDispatcher (Variables|FrameworkActors|GetAs%20BP%20GS%20Gameplay%20Server) (EventDispatchers|CreateEvent :!event Custom|On%20Show%20Result%20Board)))

(event Custom|Enable%20Visibility%20Multicast
  (Rendering|SetVisibility (Variables|Default|GetDefaultSceneRoot) true true))

(event EventBeginPlay
  (Rendering|SetVisibility (Variables|Default|GetDefaultSceneRoot) false true)
  (if (Networking|IsServer)
    (CallFunction|InitFrameworkActors)))

(fn ConstructionScript)