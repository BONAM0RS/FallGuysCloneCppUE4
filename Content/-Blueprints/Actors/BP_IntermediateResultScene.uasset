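; Between-round results stage that lines players up on 60 arrow-marked cube slots and reveals who is out and who qualifies.
; When the game state signals the result board, it lists players to kick from player states and the level's trigger type.
; A looping timer drops them one by one via multicast cube moves and ragdolls, updating the remaining count.
; It then turns qualified slots green and has the game mode schedule the next-level widget.
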(event Custom|Fill%20Arrays
  (Variables|SlotArrays|SetArrowPlayerSlots (Utilities|Array|MakeArray (Variables|Default|GetArrow) (Variables|Default|GetArrow1) (Variables|Default|GetArrow2) (Variables|Default|GetArrow3) (Variables|Default|GetArrow4) (Variables|Default|GetArrow5) (Variables|Default|GetArrow6) (Variables|Default|GetArrow7) (Variables|Default|GetArrow8) (Variables|Default|GetArrow9) (Variables|Default|GetArrow10) (Variables|Default|GetArrow11) (Variables|Default|GetArrow12) (Variables|Default|GetArrow13) (Variables|Default|GetArrow14) (Variables|Default|GetArrow15) (Variables|Default|GetArrow16) (Variables|Default|GetArrow17) (Variables|Default|GetArrow18) (Variables|Default|GetArrow19) (Variables|Default|GetArrow20) (Variables|Default|GetArrow21) (Variables|Default|GetArrow22) (Variables|Default|GetArrow23) (Variables|Default|GetArrow24) (Variables|Default|GetArrow25) (Variables|Default|GetArrow26) (Variables|Default|GetArrow27) (Variables|Default|GetArrow28) (Variables|Default|GetArrow29) (Variables|Default|GetArrow30) (Variables|Default|GetArrow31) (Variables|Default|GetArrow32) (Variables|Default|GetArrow33) (Variables|Default|GetArrow34) (Variables|Default|GetArrow35) (Variables|Default|GetArrow36) (Variables|Default|GetArrow37) (Variables|Default|GetArrow38) (Variables|Default|GetArrow39) (Variables|Default|GetArrow40) (Variables|Default|GetArrow41) (Variables|Default|GetArrow42) (Variables|Default|GetArrow43) (Variables|Default|GetArrow44) (Variables|Default|GetArrow45) (Variables|Default|GetArrow46) (Variables|Default|GetArrow47) (Variables|Default|GetArrow48) (Variables|Default|GetArrow49) (Variables|Default|GetArrow50) (Variables|Default|GetArrow51) (Variables|Default|GetArrow52) (Variables|Default|GetArrow53) (Variables|Default|GetArrow54) (Variables|Default|GetArrow55) (Variables|Default|GetArrow56) (Variables|Default|GetArrow57) (Variables|Default|GetArrow58) (Variables|Default|GetArrow59)))
  (Variables|SlotArrays|SetSlotCubes (Utilities|Array|MakeArray (Variables|Default|GetSM_Cube) (Variables|Default|GetSM_Cube1) (Variables|Default|GetSM_Cube2) (Variables|Default|GetSM_Cube3) (Variables|Default|GetSM_Cube4) (Variables|Default|GetSM_Cube5) (Variables|Default|GetSM_Cube6) (Variables|Default|GetSM_Cube7) (Variables|Default|GetSM_Cube8) (Variables|Default|GetSM_Cube9) (Variables|Default|GetSM_Cube10) (Variables|Default|GetSM_Cube11) (Variables|Default|GetSM_Cube12) (Variables|Default|GetSM_Cube13) (Variables|Default|GetSM_Cube14) (Variables|Default|GetSM_Cube15) (Variables|Default|GetSM_Cube16) (Variables|Default|GetSM_Cube17) (Variables|Default|GetSM_Cube18) (Variables|Default|GetSM_Cube19) (Variables|Default|GetSM_Cube20) (Variables|Default|GetSM_Cube21) (Variables|Default|GetSM_Cube22) (Variables|Default|GetSM_Cube23) (Variables|Default|GetSM_Cube24) (Variables|Default|GetSM_Cube25) (Variables|Default|GetSM_Cube26) (Variables|Default|GetSM_Cube27) (Variables|Default|GetSM_Cube28) (Variables|Default|GetSM_Cube29) (Variables|Default|GetSM_Cube30) (Variables|Default|GetSM_Cube31) (Variables|Default|GetSM_Cube32) (Variables|Default|GetSM_Cube33) (Variables|Default|GetSM_Cube34) (Variables|Default|GetSM_Cube35) (Variables|Default|GetSM_Cube36) (Variables|Default|GetSM_Cube37) (Variables|Default|GetSM_Cube38) (Variables|Default|GetSM_Cube39) (Variables|Default|GetSM_Cube40) (Variables|Default|GetSM_Cube41) (Variables|Default|GetSM_Cube42) (Variables|Default|GetSM_Cube43) (Variables|Default|GetSM_Cube44) (Variables|Default|GetSM_Cube45) (Variables|Default|GetSM_Cube46) (Variables|Default|GetSM_Cube47) (Variables|Default|GetSM_Cube48) (Variables|Default|GetSM_Cube49) (Variables|Default|GetSM_Cube50) (Variables|Default|GetSM_Cube51) (Variables|Default|GetSM_Cube52) (Variables|Default|GetSM_Cube53) (Variables|Default|GetSM_Cube54) (Variables|Default|GetSM_Cube55) (Variables|Default|GetSM_Cube56) (Variables|Default|GetSM_Cube57) (Variables|Default|GetSM_Cube58) (Variables|Default|GetSM_Cube59))))

(event Custom|Update%20Text%20Multicast
  (params (Number :type String) (Text :type String) (Board%20Color :type Material%20Interface%20Object%20Reference))
  (Rendering|Components|TextRender|SetText (Variables|Default|GetResultTextRender) (Utilities|Text|ToText(String) (Utilities|String|MakeLiteralString (Utilities|String|Append Number Text))))
  (Rendering|Material|SetMaterial (Variables|Default|GetSM_ResultsBoard) 0 Board%20Color))

(event Custom|Kick%20Disquilified%20Player
  (bind _players_count_to_kick (Variables|Default|GetPlayers%20Count%20To%20Kick))
  (bind _slotcubes (Variables|SlotArrays|GetSlotCubes))
  (bind _as_bp_gs_gameplay_server (Variables|Default|GetAs%20BP%20GS%20Gameplay%20Server))
  (bind _player_indexes_to_kick (Variables|Default|GetPlayer%20Indexes%20To%20Kick))
  (bind _output (Utilities|Array|Get(acopy) _player_indexes_to_kick _players_count_to_kick))
  (bind _playerarray (Variables|/Script/Engine.GameStateBase|GetPlayerArray _as_bp_gs_gameplay_server))
  (bind _output_2 (Utilities|Array|Get(acopy) _playerarray _output))
  (bind _output_3 (Utilities|Array|Get(acopy) _slotcubes _output))
  (bind _relativelocation (Variables|/Script/Engine.SceneComponent|GetRelativeLocation _output_3))
  (if (!= (Variables|Default|GetPlayers%20Count%20To%20Kick) (Utilities|Array|Length _player_indexes_to_kick))
    (Utilities|Casting|CastToBP_PS_Gameplay _output_2)
    (bind _asbp_char_gameplay (Utilities|Casting|CastToBP_Char_Gameplay (Variables|/Script/Engine.PlayerState|GetPawnPrivate _output_2)))
    (CallFunction|MoveComponenttoMulticast (Variables|/Script/Engine.Character|GetMesh _asbp_char_gameplay) (Variables|/Game/-Blueprints/-Gameplay/Core/BP_Char_Gameplay.BP_Char_Gameplay_C|GetPlayerNameWidget _asbp_char_gameplay) _output_3 (.y _relativelocation) (.z _relativelocation))
    (Math|Integer|IncrementInt (Variables|Default|GetPlayers%20Count%20To%20Kick)
      (:%20%20
        (CallFunction|UpdateTextMulticast (Utilities|String|ToString(Integer) (- (Utilities|Array|Length (Variables|/Script/Engine.GameStateBase|GetPlayerArray (Game|GetGameState))) (Utilities|Array|Length (Variables|Default|GetPlayer%20Indexes%20To%20Kick)))) " REMAIN!" "/Game/Materials/M_Pink.M_Pink")
        (CallFunction|CheckConditiontoDetermineDisqualifiedPlayersAreKicked)))))

(event Custom|Check%20Condition%20To%20Determine%20Disqualified%20Players%20Are%20Kicked
  (if (== (Variables|Default|GetPlayers%20Count%20To%20Kick) (Utilities|Array|Length (Variables|Default|GetPlayer%20Indexes%20To%20Kick)))
    (CallFunction|CreateTimertoShowQualifiedPlayers)))

(event Custom|Create%20Timer%20To%20Show%20Qualified%20Players
  (bind _returnvalue (Utilities|Time|SetTimerbyEvent (EventDispatchers|CreateEvent :!event Custom|Show%20Qualified%20Players) 2.0))
  (Variables|Timers|SetShow%20Qualified%20Players%20Timer _returnvalue))

(event Custom|Create%20Kick%20Disqualified%20Player%20Timer
  (bind _returnvalue (Utilities|Time|SetTimerbyEvent (EventDispatchers|CreateEvent :!event Custom|Kick%20Disquilified%20Player) (Variables|Default|GetLooping%20Time%20To%20Kick%20Disqualified%20Player) true (Variables|Default|GetInitial%20Start%20Delay%20To%20Kick%20Disqualified%20Players)))
  (Variables|Timers|SetKick%20Disquialified%20Players%20Timer _returnvalue))

(event Custom|Show%20Qualified%20Players
  (CallFunction|OnShowQualifiedPlayers)
  (CallFunction|UpdateTextMulticast (Utilities|String|ToString(Integer) (- (Utilities|Array|Length (Variables|/Script/Engine.GameStateBase|GetPlayerArray (Game|GetGameState))) (Utilities|Array|Length (Variables|Default|GetPlayer%20Indexes%20To%20Kick)))) " QUALIFIED!" "/Game/Materials/M_Green.M_Green")
  (for (_array_element _array_index) (Variables|/Script/Engine.GameStateBase|GetPlayerArray (Variables|Default|GetAs%20BP%20GS%20Gameplay%20Server))
    (bind _asbp_ps_gameplay (Utilities|Casting|CastToBP_PS_Gameplay _array_element))
    (if (Utilities|Enum|Equal(Enum) (Variables|/Game/-Blueprints/-Gameplay/Core/BP_PS_Gameplay.BP_PS_Gameplay_C|GetPlayer%20State _asbp_ps_gameplay) (Utilities|Enum|LiteralenumEnum_PlayerStates "NewEnumerator1"))
      (CallFunction|UpdateMaterialColorMulticast (Utilities|Array|Get(acopy) (Variables|SlotArrays|GetSlotCubes) _array_index) "/Game/Materials/M_Green.M_Green"))))

(event Custom|Update%20Material%20Color%20Multicast
  (params (Component :type Primitive%20Component%20Object%20Reference) (Material :type Material%20Interface%20Object%20Reference))
  (Rendering|Material|SetMaterial Component 0 Material))

(event Custom|On%20Show%20Qualified%20Players
  (Default|CreateTimertoShowNextLevelWidget (Variables|Default|GetAs%20BP%20GM%20Gameplay%20Server)))

(event Custom|Calculate%20Disqualified%20Players
  (bind _player_state_trigger_type (CallFunction|GetCurrentLevelInfoRowData))
  (switch Utilities|FlowControl|Switch|SwitchonEnum_LevelPlayerStateTriggerTypes _player_state_trigger_type
    (:NewEnumerator0
      (for (_array_element _array_index) (Variables|/Script/Engine.GameStateBase|GetPlayerArray (Game|GetGameState))
        (bind _asbp_ps_gameplay (Utilities|Casting|CastToBP_PS_Gameplay _array_element))
        (if (Utilities|Enum|NotEqual(Enum) (Variables|/Game/-Blueprints/-Gameplay/Core/BP_PS_Gameplay.BP_PS_Gameplay_C|GetPlayer%20State _asbp_ps_gameplay) (Utilities|Enum|LiteralenumEnum_PlayerStates "NewEnumerator2"))
          (Utilities|Array|Add (Variables|Default|GetPlayer%20Indexes%20To%20Kick) _array_index))))
    (:NewEnumerator1
      (for (_array_element_2 _array_index_2) (Variables|/Script/Engine.GameStateBase|GetPlayerArray (Game|GetGameState))
        (bind _asbp_ps_gameplay_2 (Utilities|Casting|CastToBP_PS_Gameplay _array_element_2))
        (if (Utilities|Enum|Equal(Enum) (Variables|/Game/-Blueprints/-Gameplay/Core/BP_PS_Gameplay.BP_PS_Gameplay_C|GetPlayer%20State _asbp_ps_gameplay_2) (Utilities|Enum|LiteralenumEnum_PlayerStates "NewEnumerator2"))
          (Utilities|Array|Add (Variables|Default|GetPlayer%20Indexes%20To%20Kick) _array_index_2))))))

(event Custom|Move%20Component%20To%20Multicast
  (params (Player%20Mesh :type Primitive%20Component%20Object%20Reference) (NameWIdget :type Scene%20Component%20Object%20Reference) (Component :type Primitive%20Component%20Object%20Reference) (Target%20Relative%20Location%20Y :type Float%20%28single-precision%29) (Target%20Relative%20Location%20Z :type Float%20%28single-precision%29))
  (Rendering|Material|SetMaterial Component 0 "/Game/Materials/M_Pink.M_Pink")
  (Components|MoveComponentTo Component (Math|Vector|MakeVector 0.0 Target%20Relative%20Location%20Y Target%20Relative%20Location%20Z) "0, 0, 0" false false 0.1 false)
  (Physics|SetSimulatePhysics Player%20Mesh true)
  (Collision|SetCollisionProfileName Player%20Mesh "Ragdoll" true :!class /Script/Engine.PrimitiveComponent)
  (Rendering|SetVisibility NameWIdget false false))

(event EventBeginPlay
  (|CallParentFunction)
  (CallFunction|FillArrays))

(event EventDestroyed
  (Utilities|Time|ClearandInvalidateTimerbyHandle (Variables|Timers|GetKick%20Disquialified%20Players%20Timer))
  (Utilities|Time|ClearandInvalidateTimerbyHandle (Variables|Timers|GetShow%20Qualified%20Players%20Timer)))

(event EventOnShowResultBoard
  (|CallParentFunction)
  (CallFunction|CalculateDisqualifiedPlayers)
  (CallFunction|CreateKickDisqualifiedPlayerTimer))

(event EventPlacePlayers
  (|CallParentFunction)
  (CallFunction|UpdateTextMulticast (Utilities|String|ToString(Integer) (Utilities|Array|Length (Variables|/Script/Engine.GameStateBase|GetPlayerArray (Game|GetGameState)))) " REMAIN!" "/Game/Materials/M_Pink.M_Pink")
  (for _array_element (Variables|/Script/Engine.GameStateBase|GetPlayerArray (Game|GetGameState))
    (bind _asbp_ps_gameplay (Utilities|Casting|CastToBP_PS_Gameplay _array_element))
    (if (not (Pawn|IsLocalController (Variables|/Game/-Blueprints/-Gameplay/Core/BP_PS_Gameplay.BP_PS_Gameplay_C|GetAs%20BP%20PC%20Gameplay%20Server _asbp_ps_gameplay)))
      (bind _asbp_char_gameplay (Utilities|Casting|CastToBP_Char_Gameplay (Variables|/Script/Engine.PlayerState|GetPawnPrivate _asbp_ps_gameplay) :!label _label))
      (Default|EnableCharacterVisibilityandCollisionMulticast _asbp_char_gameplay)
      (Default|TeleportPlayerMulticast _asbp_char_gameplay (Transformation|GetWorldLocation (Utilities|Array|Get(acopy) (Variables|SlotArrays|GetArrowPlayerSlots) (Variables|/Game/-Blueprints/-Gameplay/Core/BP_PS_Gameplay.BP_PS_Gameplay_C|GetPlayer%20Index _asbp_ps_gameplay))) (Transformation|GetWorldRotation (Utilities|Array|Get(acopy) (Variables|SlotArrays|GetArrowPlayerSlots) (Variables|/Game/-Blueprints/-Gameplay/Core/BP_PS_Gameplay.BP_PS_Gameplay_C|GetPlayer%20Index _asbp_ps_gameplay))))
      (elif (not (Variables|/Game/-Blueprints/-General/Core/BP_GameInstance.BP_GameInstance_C|GetisHostDisqualified (Variables|FrameworkActors|GetAs%20BP%20Game%20Instance%20Server)))
        (goto _label)))))

(event EventInitFrameworkActors
  (|CallParentFunction)
  (bind _asbp_game_instance (Utilities|Casting|CastToBP_GameInstance (Game|GetGameInstance))
    (:then
      (Variables|FrameworkActors|SetAs%20BP%20Game%20Instance%20Server _asbp_game_instance))
    (:CastFailed
      (CallFunction|PrintCastFailed self "BP_GameInstance" true true))))

(event EventBindEvents
  (|CallParentFunction)
  (EventDispatchers|BindEventtoOnRoundShowIntermediateResultScene (Variables|Default|GetAs%20BP%20GS%20Gameplay%20Server) (delegate EventOnShowResultBoard)))

(fn ConstructionScript)