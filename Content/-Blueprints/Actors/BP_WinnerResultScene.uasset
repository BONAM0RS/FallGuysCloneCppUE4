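; Winner result scene actor, a child of a shared result scene base, that shows the round winner and ends the match flow.
; It binds the parent's result board event to the game state's show-winner-scene dispatcher.
; Placing players makes characters in one specific player state visible and collidable, then teleports them by multicast to a single arrow slot.
; Showing the board also starts the game mode's timer to send all players to the menu.
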(event EventBeginPlay
  (|CallParentFunction))

(event EventOnShowResultBoard
  (|CallParentFunction)
  (Default|CreateTimertoSendAllPlayerstoMenu (Variables|Default|GetAs%20BP%20GM%20Gameplay%20Server)))

(event EventPlacePlayers
  (bind _arrowplayerslot (Variables|Default|GetArrowPlayerSlot))
  (|CallParentFunction)
  (for _array_element (Variables|/Script/Engine.GameStateBase|GetPlayerArray (Game|GetGameState))
    (bind _asbp_ps_gameplay (Utilities|Casting|CastToBP_PS_Gameplay _array_element))
    (if (Utilities|Enum|Equal(Enum) (Variables|/Game/-Blueprints/-Gameplay/Core/BP_PS_Gameplay.BP_PS_Gameplay_C|GetPlayer%20State _asbp_ps_gameplay) (Utilities|Enum|LiteralenumEnum_PlayerStates "NewEnumerator1"))
      (bind _asbp_char_gameplay (Utilities|Casting|CastToBP_Char_Gameplay (Variables|/Script/Engine.PlayerState|GetPawnPrivate _asbp_ps_gameplay)))
      (Default|EnableCharacterVisibilityandCollisionMulticast _asbp_char_gameplay)
      (Default|TeleportPlayerMulticast _asbp_char_gameplay (Transformation|GetWorldLocation _arrowplayerslot) (Transformation|GetWorldRotation _arrowplayerslot)))))

(event EventBindEvents
  (|CallParentFunction)
  (EventDispatchers|BindEventtoOnRoundShowWinnerResultScene (Variables|Default|GetAs%20BP%20GS%20Gameplay%20Server) (delegate EventOnShowResultBoard)))

(fn ConstructionScript)