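; BP_PlayerState holds a player's name and match status: None, Play, Qualified or Disqualified.
; On BeginPlay it loads the "info" save slot as BP_SaveGame, passes the saved PlayerName to SendNameToServer to store as Name, then resets State to None.
; The SetState event maps an incoming player state onto State.
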(event Custom|SetState
  (params (PlayerState :type Enum_PlayerState%20Enum :default "NewEnumerator0"))
  (switch Utilities|FlowControl|Switch|SwitchonEnum_PlayerState PlayerState
    (:NewEnumerator0
      (Variables|Default|SetState "Play"))
    (:NewEnumerator1
      (Variables|Default|SetState "Qualified"))
    (:NewEnumerator2
      (Variables|Default|SetState "Disqualified"))))

(event Custom|Send%20Name%20To%20Server
  (params (Name :type Text))
  (Variables|Default|SetName Name))

(event EventBeginPlay
  (bind _returnvalue (SaveGame|LoadGamefromSlot "info"))
  (bind _asbp_save_game (Utilities|Casting|CastToBP_SaveGame _returnvalue))
  (CallFunction|SendNametoServer (Variables|/Game/Save/BP_SaveGame.BP_SaveGame_C|GetPlayerName _asbp_save_game))
  (Variables|Default|SetState "None"))

(event EventTick
  (params (DeltaSeconds :type Float%20%28single-precision%29)))

(fn ConstructionScript)