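; Gameplay player controller that applies the saved player sex to the possessed character.
; On possess, gated to authority, it reads PlayerSex from the "info" save slot and passes it to ServerChangeSex, which sets Gender on the controlled BP_Character.
; Because of that gate, the save is read on the authority's machine.
; SetMesh forwards a given gender to the same event without touching the save.
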(event Custom|Local%20Change%20Sex
  (bind _returnvalue (SaveGame|LoadGamefromSlot "info"))
  (bind _asbp_save_game (Utilities|Casting|CastToBP_SaveGame _returnvalue))
  (CallFunction|ServerChangeSex (Variables|/Game/Save/BP_SaveGame.BP_SaveGame_C|GetPlayerSex _asbp_save_game)))

(event Custom|Server%20Change%20Sex
  (params (Gender :type Boolean))
  (bind _asbp_character (Utilities|Casting|CastToBP_Character (Pawn|GetControlledPawn)))
  (Variables|/Game/-Blueprints/Core/BP_Character.BP_Character_C|SetGender _asbp_character Gender))

(event Custom|Set%20Mesh
  (params (Gender :type Boolean))
  (CallFunction|ServerChangeSex Gender))

(event EventPossess
  (params (PossessedPawn :type Pawn%20Object%20Reference))
  (Networking|SwitchHasAuthority
    (:Authority
      (CallFunction|LocalChangeSex))))

(fn ConstructionScript)