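; BP_Char_Gameplay is a gameplay character with a player name widget and one of two body materials.
; On BeginPlay it applies the material, passes itself to the WB_PlayerName widget and disables input for player controller 0.
; UpdateMesh swaps only the material, purple or cyan by IsQuinn, and OnRep_Gender reruns it when that replicated state changes.
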(event Custom|Update%20Mesh
  (Rendering|Material|SetMaterial (Variables|Character|GetMesh) 0 (select (Variables|Default|GetIsQuinn) "/Game/Materials/M_Purple.M_Purple" "/Game/IstonArt/Materials/M_Color_Cyan.M_Color_Cyan")))

(event Custom|SetCharToPlayerNameWidget
  (bind _aswb_player_name (Utilities|Casting|CastToWB_PlayerName (UserInterface|GetUserWidgetObject (Variables|Default|GetPlayerNameWidget))))
  (Variables|/Game/-Blueprints/-Gameplay/Widgets/WB_PlayerName.WB_PlayerName_C|SetPlayerChar _aswb_player_name self))

(event EventBeginPlay
  (CallFunction|UpdateMesh)
  (CallFunction|SetChartoPlayerNameWidget)
  (Input|DisableInput (Game|GetPlayerController 0)))

(fn ConstructionScript)

(fn OnRepGender
  (CallFunction|UpdateMesh))