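; BP_HUD_Gameplay is the gameplay HUD, managing the player's on-screen widgets.
; On BeginPlay it sets game-only input, hides the cursor, adds the chat overlay and shows the FPS counter if the "info" save enables it.
; Events create or remove the players info board and toggle a test main menu.
; The menu's creation code is disconnected, so WBMenu is never assigned here.
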(event Custom|Show%20Players%20Info%20Borad
  (bind _returnvalue (UserInterface|CreateWidget "/Game/-Blueprints/-Gameplay/Widgets/PlayersInfoTab/WB_PlayersInfoBoard.WB_PlayersInfoBoard_C" (Variables|Default|GetPlayerOwner)))
  (UserInterface|Viewport|AddtoViewport _returnvalue 0))

(event Custom|Show%20Main%20Menu
  ;[1 1 1] Tested Main Menu In Gameplay
  (UserInterface|Viewport|AddtoViewport (Variables|Default|GetWB_Menu) 0)
  (Variables|Default|SetisMainMenuOpened true))

(event Custom|Hide%20Players%20Info%20Board
  (Widget|RemovefromParent (stale Custom|Show%20Players%20Info%20Borad _returnvalue)))

(event Custom|Hide%20Main%20Menu
  ;[1 1 1] Tested Main Menu In Gameplay
  (Widget|RemovefromParent (Variables|Default|GetWB_Menu))
  (Variables|Default|SetisMainMenuOpened false))

(event EventBeginPlay
  (bind _playerowner (Variables|Default|GetPlayerOwner))
  (Utilities|FlowControl|Sequence
    (:then_0
      (Input|SetInputModeGameOnly _playerowner)
      (Variables|/Script/Engine.PlayerController|SetbShowMouseCursor _playerowner false))
    (:then_1
      (bind _returnvalue (UserInterface|CreateWidget "/Game/-Blueprints/-General/Widgets/WB_FPS.WB_FPS_C" (Game|Player|GetOwningPlayerController)))
      (bind _returnvalue_2 (SaveGame|LoadGamefromSlot "info"))
      (bind _asbp_save_game (Utilities|Casting|CastToBP_SaveGame _returnvalue_2))
      (if (Variables|/Game/-Blueprints/-General/Core/BP_SaveGame.BP_SaveGame_C|GetShowFPS _asbp_save_game)
        (UserInterface|Viewport|AddtoViewport _returnvalue 0)
        (else
          (Widget|RemovefromParent _returnvalue))))
    (:then_2
      (bind _returnvalue_3 (UserInterface|CreateWidget "/Game/-Blueprints/-Gameplay/Widgets/Chat/WB_ChatOnScreen.WB_ChatOnScreen_C" (Variables|Default|GetPlayerOwner)))
      (bind _output_get (Variables|Default|SetWB_ChatOnScreen _returnvalue_3))
      (UserInterface|Viewport|AddtoViewport _output_get 0))))

(fn ConstructionScript)