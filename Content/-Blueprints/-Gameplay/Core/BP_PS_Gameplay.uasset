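; Gameplay PlayerState that tracks a player's name, character choice (IsQuinn), host flag, spectated player index and round state.
; On BeginPlay, the local player's copy pulls name and character from the GameInstance, announces the connection in chat, detects the host and binds round events.
; Round start sets the state to Play unless the host is disqualified.
; OnRep_PlayerState turns state changes into Play, Qualified, Eliminated and Spectate dispatcher calls.
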(event Custom|Set%20State
  (params (New%20Player%20State :type Enum_PlayerStates%20Enum :default "NewEnumerator5"))
  (Variables|PlayerData|SetPlayer%20State New%20Player%20State))

(event Custom|On%20Round%20FInished)

(event Custom|Set%20Spectator%20Player%20Index
  (params (New%20Spectator%20Player%20Index :type Integer))
  (Variables|PlayerData|SetSpectator%20Player%20Index New%20Spectator%20Player%20Index))

(event Custom|Init%20Game%20State
  (bind _asbp_gs_gameplay (Utilities|Casting|CastToBP_GS_Gameplay (Game|GetGameState)))
  (Variables|FrameworkActors|SetAs%20BP%20GS%20Gameplay%20Server _asbp_gs_gameplay)
  (bind _asbp_gm_gameplay (Utilities|Casting|CastToBP_GM_Gameplay (Game|GetGameMode)))
  (Variables|FrameworkActors|SetAs%20BP%20GM%20Gameplay%20Server _asbp_gm_gameplay))

(event Custom|Send%20Name%20To%20Server
  (params (Name :type Text))
  (Variables|PlayerData|SetPlayer%20Name Name)
  (bind _asbp_gm_gameplay (Utilities|Casting|CastToBP_GM_Gameplay (Game|GetGameMode)))
  (Default|SendChatMessagetoAllPlayerControllers _asbp_gm_gameplay (Utilities|String|ToString(Text) (Variables|PlayerData|GetPlayer%20Name)) " connected to server" 1))

(event Custom|Init%20Game%20Instance
  (bind _asbp_game_instance (Utilities|Casting|CastToBP_GameInstance (Game|GetGameInstance)))
  (bind _output_get (Variables|FrameworkActors|SetAs%20BP%20Game%20Instance%20Server _asbp_game_instance))
  (CallFunction|Server (Variables|/Game/-Blueprints/-General/Core/BP_GameInstance.BP_GameInstance_C|GetIsQuinn _output_get)))

(event Custom|Check%20Host
  (if (and (Networking|IsServer) (Pawn|IsLocalController (Variables|FrameworkActors|GetAs%20BP%20PC%20Gameplay%20Server)))
    (Variables|PlayerData|SetIs%20Host true)))

(event Custom|Bind%20Events
  (EventDispatchers|BindEventtoOnRoundStarted (Variables|FrameworkActors|GetAs%20BP%20GS%20Gameplay%20Server) (EventDispatchers|CreateEvent :!event Custom|On%20Round%20Started))
  (EventDispatchers|BindEventtoOnRoundFinished (Variables|FrameworkActors|GetAs%20BP%20GS%20Gameplay%20Server) (EventDispatchers|CreateEvent :!event Custom|On%20Round%20FInished))
  (EventDispatchers|BindEventtoOnPlayerQualified (EventDispatchers|CreateEvent (Variables|FrameworkActors|GetAs%20BP%20GM%20Gameplay%20Server) :!event AddPlayerStatesScore))
  (EventDispatchers|BindEventtoOnPlayerEliminated (EventDispatchers|CreateEvent (Variables|FrameworkActors|GetAs%20BP%20GM%20Gameplay%20Server) :!event AddPlayerStatesScore)))

(event Custom|On%20Round%20Started
  (Variables|PlayerData|SetPlayer%20Index (Class|GameplayStatics|GetPlayerControllerID (Variables|FrameworkActors|GetAs%20BP%20PC%20Gameplay%20Server)))
  (if (not (Variables|PlayerData|GetIs%20Host))
    (Variables|PlayerData|SetPlayer%20State "NewEnumerator0" :!label _label)
    (else
      (bind _asbp_game_instance (Utilities|Casting|CastToBP_GameInstance (Game|GetGameInstance)))
      (if (not (Variables|/Game/-Blueprints/-General/Core/BP_GameInstance.BP_GameInstance_C|GetisHostDisqualified _asbp_game_instance))
        (goto _label)))))

(event Custom|Server
  (params (Is%20Quinn :type Boolean))
  (Variables|PlayerData|SetIs%20Quinn Is%20Quinn))

(event EventBeginPlay
  (bind _asbp_pc_gameplay (Utilities|Casting|CastToBP_PC_Gameplay (Components|GetOwner)))
  (Variables|FrameworkActors|SetAs%20BP%20PC%20Gameplay%20Server _asbp_pc_gameplay)
  (if (Pawn|IsLocalPlayerController (Variables|FrameworkActors|GetAs%20BP%20PC%20Gameplay%20Server))
    (CallFunction|InitGameInstance)
    (CallFunction|SendNametoServer (Variables|/Game/-Blueprints/-General/Core/BP_GameInstance.BP_GameInstance_C|GetPlayerName (Variables|FrameworkActors|GetAs%20BP%20Game%20Instance%20Server)))
    (CallFunction|CheckHost)
    (CallFunction|InitGameState)
    (CallFunction|BindEvents)))

(fn ConstructionScript)

(fn OnRepPlayerState
  (switch Utilities|FlowControl|Switch|SwitchonEnum_PlayerStates (Variables|PlayerData|GetPlayer%20State)
    (:NewEnumerator0
      (Default|CallOnPlayerPlay))
    (:NewEnumerator1
      (Default|CallOnPlayerQualified))
    (:NewEnumerator4
      (Default|CallOnPlayerEliminated))
    (:NewEnumerator2
      (Default|CallOnPlayerSpectate))))