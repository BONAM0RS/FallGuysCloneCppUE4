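; Gameplay player controller for a round-based multiplayer game with qualification, handling HUD, menu, chat, input and spectating.
; GameState dispatchers drive player-state setup and enable input at round start, while chat toggles input mode and relays messages through GameMode and GameState.
; On possession, the client sends its GameInstance mesh choice (Quinn flag) to the server.
; Spectator mode follows qualification or host disqualification, cycling view targets through PlayerArray, skipping players not playing.
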(event Custom|SendChatMessageToGameState
  (params (Sender :type String) (Message :type String) (MessageType :type Byte))
  (bind _asbp_gs_gameplay (Utilities|Casting|CastToBP_GS_Gameplay (Game|GetGameState)))
  (Default|CallonChatMessageSendtoGameState _asbp_gs_gameplay Sender Message MessageType))

(event Custom|Init%20HUD
  (bind _asbp_hud_gameplay (Utilities|Casting|CastToBP_HUD_Gameplay (HUD|GetHUD)))
  (Variables|FrameworkActors|SetHUD%20Gameplay%20Client _asbp_hud_gameplay))

(event Custom|Select%20Previous%20Spectator%20Index
  (Variables|Default|SetIs%20Choose%20Next%20Spectator%20Player false)
  (if (== (Variables|Default|GetSpectator%20Player%20Index) 0)
    (Variables|Default|SetSpectator%20Player%20Index (- (Utilities|Array|Length (Variables|/Script/Engine.GameStateBase|GetPlayerArray (Game|GetGameState))) 1))
    (else
      (Math|Integer|DecrementInt (Variables|Default|GetSpectator%20Player%20Index)
        (:%20%20
          _))))
  (Development|PrintString (Utilities|String|Append "previous index " (Utilities|String|ToString(Integer) (Variables|Default|GetSpectator%20Player%20Index))) true true "(R=0.000000,G=0.660000,B=1.000000,A=1.000000)" 3.6e+02)
  (CallFunction|CheckSpectatorIndex))

(event Custom|Enable%20Player%20Input
  (Input|EnableInput (Pawn|GetControlledPawn) self))

(event Custom|Init%20Game%20Instance
  (bind _asbp_game_instance (Utilities|Casting|CastToBP_GameInstance (Game|GetGameInstance)))
  (Variables|FrameworkActors|SetAs%20BP%20Game%20Instance%20Client _asbp_game_instance))

(event Custom|Switch%20To%20Spectator%20Mode%20If%20Host%20And%20Was%20Disqualified%20In%20Previous%20Round
  (if (Variables|/Game/-Blueprints/-Gameplay/Core/BP_PS_Gameplay.BP_PS_Gameplay_C|GetIs%20Host (Variables|FrameworkActors|GetAs%20BP%20PS%20Gameplay))
    (bind _asbp_game_instance (Utilities|Casting|CastToBP_GameInstance (Game|GetGameInstance)))
    (if (Variables|/Game/-Blueprints/-General/Core/BP_GameInstance.BP_GameInstance_C|GetisHostDisqualified _asbp_game_instance)
      (CallFunction|EnableSpectatorMode))))

(event Custom|On%20Round%20Started
  (CallFunction|EnablePlayerInput))

(event Custom|FillSpectatingPlayerName
  (params (InText :type Text))
  (Default|FillWatchingPlayerName (Variables|/Game/-Blueprints/-Gameplay/Core/BP_HUD_Gameplay.BP_HUD_Gameplay_C|GetWB_Spectating (Variables|FrameworkActors|GetHUD%20Gameplay%20Client)) InText))

(event Custom|On%20Players%20Connected
  (CallFunction|InitPlayerState)
  (CallFunction|SwitchtoSpectatorModeifHostandWasDisqualifiedinPreviousRound)
  (CallFunction|SubscribetoEventonQualificationPopUpEnd))

(event Custom|Init%20Character%20Mesh
  (Networking|SwitchHasAuthority
    (:Authority
      (CallFunction|ClientInitCharacterMesh))))

(event Custom|Server%20Init%20Character%20Mesh
  (params (IsQuinn :type Boolean))
  (Variables|/Game/-Blueprints/-Gameplay/Core/BP_Char_Gameplay.BP_Char_Gameplay_C|SetIsQuinn (Variables|FrameworkActors|GetAs%20BP%20Char%20Gameplay) IsQuinn))

(event Custom|CallOnChatMessageSendToGameMode
  (params (Sender :type String) (Message :type String) (MessageType :type Byte))
  ;[1 1 1] From GameMode
  (Default|CallOnChatMessageSendtoGameMode Sender Message MessageType))

(event Custom|Show%20Next%20Level%20Widget%20White%20Screen
  (Widget|SetVisibility (Variables|/Game/-Blueprints/-Gameplay/Widgets/WB_NextLevel.WB_NextLevel_C|GetImage_BackgroundWhite (Variables|/Game/-Blueprints/-Gameplay/Core/BP_HUD_Gameplay.BP_HUD_Gameplay_C|GetWB_NextLevel (Variables|FrameworkActors|GetHUD%20Gameplay%20Client))) "Visible"))

(event Custom|GoToMenu
  ;[1 1 1] Inputs
  (Game|OpenLevel(byObjectReference) "/Game/-Maps/Menu/L_Menu.L_Menu"))

(event Custom|Init%20Gameplay%20Player%20State
  (params (BP%20PS%20Gameplay :type BP%20PS%20Gameplay%20Object%20Reference))
  (Variables|FrameworkActors|SetAs%20BP%20PS%20Gameplay BP%20PS%20Gameplay))

(event Custom|Subscribe%20To%20Event%20On%20Qualification%20Pop%20Up%20End
  (EventDispatchers|BindEventtoOnQualificationPopUpEnd (Variables|/Game/-Blueprints/-Gameplay/Core/BP_HUD_Gameplay.BP_HUD_Gameplay_C|GetWB_QualificataionPopUp (Variables|FrameworkActors|GetHUD%20Gameplay%20Client)) (EventDispatchers|CreateEvent :!event Custom|On%20Qualification%20Pop%20Up%20End)))

(event Custom|Init%20Player%20State
  (bind _asbp_ps_gameplay (Utilities|Casting|CastToBP_PS_Gameplay (Variables|Default|GetPlayerState)))
  (Variables|FrameworkActors|SetAs%20BP%20PS%20Gameplay _asbp_ps_gameplay))

(event Custom|Enable%20Spectator%20Mode
  (Default|CallOnEnableSpectatorMode)
  (CallFunction|CheckSpectatorIndex))

(event Custom|On%20Qualification%20Pop%20Up%20End
  (if (Utilities|Enum|NotEqual(Enum) (Variables|/Game/-Blueprints/-Gameplay/Core/BP_GS_Gameplay.BP_GS_Gameplay_C|GetRound%20State (Variables|FrameworkActors|GetAs%20BP%20GS%20Gameplay)) (Utilities|Enum|LiteralenumEnum_RoundStates "NewEnumerator2"))
    (CallFunction|EnableSpectatorMode)))

(event Custom|HideChat
  ;[1 1 1] Inputs
  (Default|HideChat (Variables|/Game/-Blueprints/-Gameplay/Widgets/Chat/WB_ChatOnScreen.WB_ChatOnScreen_C|GetWB_ChatBox (Variables|/Game/-Blueprints/-Gameplay/Core/BP_HUD_Gameplay.BP_HUD_Gameplay_C|GetWB_ChatOnScreen (Variables|FrameworkActors|GetHUD%20Gameplay%20Client))))
  (Variables|Default|SetbShowMouseCursor false)
  (Input|SetInputModeGameOnly self)
  (bind _asbp_gs_gameplay (Utilities|Casting|CastToBP_GS_Gameplay (Game|GetGameState)))
  (if (Utilities|Enum|Equal(Enum) (Variables|/Game/-Blueprints/-Gameplay/Core/BP_GS_Gameplay.BP_GS_Gameplay_C|GetRound%20State _asbp_gs_gameplay) (Utilities|Enum|LiteralenumEnum_RoundStates "NewEnumerator1"))
    (Input|EnableInput (Pawn|GetControlledPawn) self)))

(event Custom|Client%20Init%20Character%20Mesh
  (CallFunction|InitGameInstance)
  (CallFunction|ServerInitCharacterMesh (Variables|/Game/-Blueprints/-General/Core/BP_GameInstance.BP_GameInstance_C|GetIsQuinn (Variables|FrameworkActors|GetAs%20BP%20Game%20Instance%20Client))))

(event Custom|Check%20Spectator%20Index
  (bind _returnvalue (Game|GetGameState))
  (bind _spectator_player_index (Variables|Default|GetSpectator%20Player%20Index))
  (bind _playerarray (Variables|/Script/Engine.GameStateBase|GetPlayerArray _returnvalue))
  (bind _output (Utilities|Array|Get(acopy) _playerarray _spectator_player_index))
  (bind _asbp_ps_gameplay (Utilities|Casting|CastToBP_PS_Gameplay _output))
  (if (Utilities|Enum|Equal(Enum) (Variables|/Game/-Blueprints/-Gameplay/Core/BP_PS_Gameplay.BP_PS_Gameplay_C|GetPlayer%20State _asbp_ps_gameplay) (Utilities|Enum|LiteralenumEnum_PlayerStates "NewEnumerator0"))
    (Game|Player|SetViewTargetwithBlend self (Variables|/Script/Engine.PlayerState|GetPawnPrivate _output) 0.0 "VTBlend_Linear" 0.0 false)
    (CallFunction|FillSpectatingPlayerName self (Variables|/Game/-Blueprints/-Gameplay/Core/BP_PS_Gameplay.BP_PS_Gameplay_C|GetPlayer%20Name _asbp_ps_gameplay))
    (else
      (Development|PrintString "Choose PlayerState that not equils PLAY" true true "(R=1.000000,G=0.000000,B=0.027276,A=1.000000)" 3.6e+02)
      (if (Variables|Default|GetIs%20Choose%20Next%20Spectator%20Player)
        (CallFunction|SelectNextSpectatorIndex)
        (else
          (CallFunction|SelectPreviousSpectatorIndex))))))

(event Custom|SendChatMessageToGameMode
  (params (Sender :type String) (Message :type String) (MessageType :type Byte))
  (bind _asbp_gm_gameplay (Utilities|Casting|CastToBP_GM_Gameplay (Game|GetGameMode)))
  (Default|SendChatMessagetoAllPlayerControllers _asbp_gm_gameplay Sender Message MessageType))

(event Custom|Choose%20Random%20Spectator%20Index
  (Variables|Default|SetSpectator%20Player%20Index (Math|Random|RandomIntegerinRange (Variables|Default|GetSpectator%20Player%20Index) (- (Utilities|Array|Length (Variables|/Script/Engine.GameStateBase|GetPlayerArray (Game|GetGameState))) 1)))
  (CallFunction|CheckSpectatorIndex))

(event Custom|Select%20Next%20Spectator%20Index
  (Variables|Default|SetIs%20Choose%20Next%20Spectator%20Player true)
  (if (== (Variables|Default|GetSpectator%20Player%20Index) (- (Utilities|Array|Length (Variables|/Script/Engine.GameStateBase|GetPlayerArray (Game|GetGameState))) 1))
    (Variables|Default|SetSpectator%20Player%20Index 0)
    (else
      (Math|Integer|IncrementInt (Variables|Default|GetSpectator%20Player%20Index)
        (:%20%20
          _))))
  (Development|PrintString (Utilities|String|Append "next index " (Utilities|String|ToString(Integer) (Variables|Default|GetSpectator%20Player%20Index))) true true "(R=0.000000,G=0.660000,B=1.000000,A=1.000000)" 3.6e+02)
  (CallFunction|CheckSpectatorIndex))

(event EventPossess
  (params (PossessedPawn :type Pawn%20Object%20Reference))
  (bind _asbp_char_gameplay (Utilities|Casting|CastToBP_Char_Gameplay PossessedPawn)
    (:then
      (Variables|FrameworkActors|SetAs%20BP%20Char%20Gameplay _asbp_char_gameplay)
      (CallFunction|InitCharacterMesh))
    (:CastFailed
      (CallFunction|PrintCastFailed self _asbp_char_gameplay true true))))

(event EventBeginPlay
  (CallFunction|InitHUD)
  (Variables|/Script/Engine.PlayerController|SetbShowMouseCursor self false)
  (Input|SetInputModeGameOnly self)
  (bind _asbp_gs_gameplay (Utilities|Casting|CastToBP_GS_Gameplay (Game|GetGameState)))
  (Variables|FrameworkActors|SetAs%20BP%20GS%20Gameplay _asbp_gs_gameplay)
  (EventDispatchers|BindEventtoOnPlayersConnectedDispatcher (Variables|FrameworkActors|GetAs%20BP%20GS%20Gameplay) (EventDispatchers|CreateEvent :!event Custom|On%20Players%20Connected))
  (EventDispatchers|BindEventtoOnRoundStartedDispatcher (Variables|FrameworkActors|GetAs%20BP%20GS%20Gameplay) (EventDispatchers|CreateEvent :!event Custom|On%20Round%20Started)))

(event Input|ActionEvents|InputActionOpenPlayerInfoBorad
  (params (Key :type Key%20Structure :default "None"))
  (bind _hud_gameplay_client (Variables|FrameworkActors|GetHUD%20Gameplay%20Client))
  ;[1 1 1] Inputs
  (:Pressed
    (Default|ShowPlayersInfoBorad _hud_gameplay_client))
  (:Released
    (Default|HidePlayersInfoBoard _hud_gameplay_client)))

(event Input|ActionEvents|InputActionOpenChat
  (params (Key :type Key%20Structure :default "None"))
  (bind _returnvalue (Pawn|GetControlledPawn))
  (bind _self self)
  (bind _self_2 self)
  (bind _hud_gameplay_client (Variables|FrameworkActors|GetHUD%20Gameplay%20Client))
  (bind _wb_chatonscreen (Variables|/Game/-Blueprints/-Gameplay/Core/BP_HUD_Gameplay.BP_HUD_Gameplay_C|GetWB_ChatOnScreen _hud_gameplay_client))
  (bind _wb_chatbox (Variables|/Game/-Blueprints/-Gameplay/Widgets/Chat/WB_ChatOnScreen.WB_ChatOnScreen_C|GetWB_ChatBox _wb_chatonscreen))
  ;[1 1 1] Inputs
  (:Pressed
    (if (== (Class|WidgetSwitcher|GetActiveWidgetIndex (Variables|/Game/-Blueprints/-Gameplay/Widgets/Chat/WB_ChatBox.WB_ChatBox_C|GetWidgetSwitcher_0 (Variables|/Game/-Blueprints/-Gameplay/Widgets/Chat/WB_ChatOnScreen.WB_ChatOnScreen_C|GetWB_ChatBox _wb_chatonscreen))) 0)
      (Default|ShowChat _wb_chatbox)
      (Variables|Default|SetbShowMouseCursor true)
      (Input|SetInputModeGameandUI _self (Variables|/Game/-Blueprints/-Gameplay/Widgets/Chat/WB_ChatBox.WB_ChatBox_C|GetEditableTextBox_Message _wb_chatbox) "DoNotLock" true)
      (Input|DisableInput _returnvalue _self_2)
      (else
        (Default|HideChat _wb_chatbox)
        (Variables|Default|SetbShowMouseCursor false)
        (Input|SetInputModeGameOnly _self)
        (bind _asbp_gs_gameplay (Utilities|Casting|CastToBP_GS_Gameplay (Game|GetGameState)))
        (if (Utilities|Enum|Equal(Enum) (Variables|/Game/-Blueprints/-Gameplay/Core/BP_GS_Gameplay.BP_GS_Gameplay_C|GetRound%20State _asbp_gs_gameplay) (Utilities|Enum|LiteralenumEnum_RoundStates "NewEnumerator1"))
          (Input|EnableInput _returnvalue _self_2))))))

(event Input|ActionEvents|InputActionSelectNextSpectatorPlayerIndex
  (params (Key :type Key%20Structure :default "None"))
  (:Pressed
    (if (Variables|/Game/-Blueprints/-Gameplay/Core/BP_PS_Gameplay.BP_PS_Gameplay_C|GetIs%20Spectator (Variables|FrameworkActors|GetAs%20BP%20PS%20Gameplay))
      (CallFunction|SelectNextSpectatorIndex))))

(event Input|ActionEvents|InputActionSelectPreviousSpectatorPlayerIndex
  (params (Key :type Key%20Structure :default "None"))
  (:Pressed
    (if (Variables|/Game/-Blueprints/-Gameplay/Core/BP_PS_Gameplay.BP_PS_Gameplay_C|GetIs%20Spectator (Variables|FrameworkActors|GetAs%20BP%20PS%20Gameplay))
      (CallFunction|SelectPreviousSpectatorIndex))))

(event Input|ActionEvents|InputActionOpenMenu
  (params (Key :type Key%20Structure :default "None"))
  ;[1 1 1] Inputs
  (:Pressed
    (Game|OpenLevel(byObjectReference) "/Game/-Maps/Menu/L_Menu.L_Menu")))

(fn ConstructionScript)