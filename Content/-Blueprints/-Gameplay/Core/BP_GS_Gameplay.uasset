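; Game state that runs a multiplayer elimination round from waiting for players to travel to the next level.
; Chained one-second server timers drive ready check, start countdown, results or winner board, and next-level travel.
; The level's win condition sets a qualification target that ends the round when reached, marking losers disqualified.
; A disqualified host stays as spectator while others return to menu; RepNotifies broadcast score and countdown changes.
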(event Custom|CheckConditionToPlayersReady
  (bind _mincounttimetoplayersready (Variables|Default|GetMinCountTimeToPlayersReady))
  (Development|PrintString (Utilities|String|ToString(Integer) _mincounttimetoplayersready) true true "(R=1.000000,G=0.651462,B=0.028789,A=1.000000)" 3.6e+02)
  (if (or (and (== _mincounttimetoplayersready 0) (== (Utilities|Array|Length (Variables|Default|GetPlayerArray)) (Variables|/Game/-Blueprints/-General/Core/BP_GameInstance.BP_GameInstance_C|GetPlayersConnectedToSession (Variables|Default|GetAs%20BP%20Game%20Instance%20Server)))) (== (Variables|Default|GetMaxCountTimeToPlayersReady) 0))
    (if (!= (Variables|Default|GetMaxQualificationInfoScore) 0)
      _
      (else
        (Variables|Default|SetMaxQualificationInfoScore 1)))
    (bind _returnvalue (Utilities|Time|SetTimerbyEvent (EventDispatchers|CreateEvent :!event Custom|UpdateStartCountTime) 1.0 true))
    (Variables|Default|SetStartGameTimer _returnvalue)
    (for _array_element (Variables|Default|GetPlayerArray)
      (bind _asbp_pc_gameplay (Utilities|Casting|CastToBP_PC_Gameplay (Components|GetOwner _array_element))
        (:then
          (Default|HideWaitingforPlayersWidget _asbp_pc_gameplay)
          (if (Pawn|IsLocalController _asbp_pc_gameplay)
            (bind _asbp_ps_gameplay (Utilities|Casting|CastToBP_PS_Gameplay _array_element))
            (Variables|/Game/-Blueprints/-Gameplay/Core/BP_PS_Gameplay.BP_PS_Gameplay_C|SetisHost _asbp_ps_gameplay true)
            (if (Variables|/Game/-Blueprints/-General/Core/BP_GameInstance.BP_GameInstance_C|GetisHostDisqualified (Variables|Default|GetAs%20BP%20Game%20Instance%20Server))
              (bind _asbp_char_gameplay (Utilities|Casting|CastToBP_Char_Gameplay (Variables|/Script/Engine.PlayerState|GetPawnPrivate _asbp_ps_gameplay)))
              (Default|DisableVisibilityandCollisionMulticast _asbp_char_gameplay)
              (Default|DisablePlayerInput _asbp_char_gameplay)
              (Default|ChooseNextSpectatorIndex _asbp_ps_gameplay)
              (Default|ShowSpectatingWidget _asbp_pc_gameplay))))
        (:CastFailed
          (CallFunction|PrintCastFailed self 0 true true))))))

(event Custom|UpdateReadyCountTime
  (if (!= (Variables|Default|GetMinCountTimeToPlayersReady) 0)
    (Math|Integer|DecrementInt (Variables|Default|GetMinCountTimeToPlayersReady)
      (:%20%20
        (Math|Integer|DecrementInt (Variables|Default|GetMaxCountTimeToPlayersReady)
          (:%20%20
            (CallFunction|CheckConditiontoPlayersReady)))))))

(event Custom|Send%20Players%20To%20Menu
  (for _array_element (Variables|Default|GetPlayerArray)
    (bind _asbp_pc_gameplay (Utilities|Casting|CastToBP_PC_Gameplay (Components|GetOwner _array_element)))
    (if (not (Pawn|IsLocalController _asbp_pc_gameplay))
      (Default|GotoMenu _asbp_pc_gameplay)))
  (bind _asbp_pc_gameplay_2 (Utilities|Casting|CastToBP_PC_Gameplay (Components|GetOwner (Utilities|Array|Get(acopy) (Variables|Default|GetPlayerArray)))))
  (Default|GotoMenu _asbp_pc_gameplay_2))

(event Custom|Check%20Finish%20Round%20Condition
  (if (== (Variables|Default|GetCurrentQualificationInfoScore) (Variables|Default|GetMaxQualificationInfoScore))
    (Variables|Default|SetisRoundOver true)
    (CallFunction|FinishRound)))

(event Custom|Disqualify%20Players%20Loosers
  (bind _qualification_info_type (CallFunction|GetCurrentLevelInfoRowData))
  (if (Utilities|Enum|NotEqual(Enum) _qualification_info_type (Utilities|Enum|LiteralenumEnum_LevelQualificationInfoTypes "NewEnumerator1"))
    (for (_array_element _array_index) (Variables|Default|GetPlayerArray)
      (bind _asbp_ps_gameplay (Utilities|Casting|CastToBP_PS_Gameplay _array_element))
      (if (Utilities|Enum|Equal(Enum) (Variables|/Game/-Blueprints/-Gameplay/Core/BP_PS_Gameplay.BP_PS_Gameplay_C|GetPlayerState _asbp_ps_gameplay) (Utilities|Enum|LiteralenumEnum_PlayerStates "NewEnumerator0"))
        (Variables|/Game/-Blueprints/-Gameplay/Core/BP_PS_Gameplay.BP_PS_Gameplay_C|SetPlayerState _asbp_ps_gameplay "NewEnumerator2")
        (if (Variables|/Game/-Blueprints/-Gameplay/Core/BP_PS_Gameplay.BP_PS_Gameplay_C|GetisHost _asbp_ps_gameplay)
          (if (not (Variables|/Game/-Blueprints/-General/Core/BP_GameInstance.BP_GameInstance_C|GetisHostDisqualified (Variables|Default|GetAs%20BP%20Game%20Instance%20Server)))
            (Variables|/Game/-Blueprints/-General/Core/BP_GameInstance.BP_GameInstance_C|SetisHostDisqualified (Variables|Default|GetAs%20BP%20Game%20Instance%20Server) true)
            (Utilities|Array|Add (Variables|Default|GetDisqualifiedPlayersIndexesToKick) _array_index :!label _label))
          (else
            (goto _label)))))
    (else
      (for (_array_element_2 _array_index_2) (Variables|Default|GetPlayerArray)
        (bind _asbp_ps_gameplay_2 (Utilities|Casting|CastToBP_PS_Gameplay _array_element_2))
        (if (Utilities|Enum|Equal(Enum) (Variables|/Game/-Blueprints/-Gameplay/Core/BP_PS_Gameplay.BP_PS_Gameplay_C|GetPlayerState _asbp_ps_gameplay_2) (Utilities|Enum|LiteralenumEnum_PlayerStates "NewEnumerator4"))
          (Variables|/Game/-Blueprints/-Gameplay/Core/BP_PS_Gameplay.BP_PS_Gameplay_C|SetPlayerState _asbp_ps_gameplay_2 "NewEnumerator2")
          (if (Variables|/Game/-Blueprints/-Gameplay/Core/BP_PS_Gameplay.BP_PS_Gameplay_C|GetisHost _asbp_ps_gameplay_2)
            (if (not (Variables|/Game/-Blueprints/-General/Core/BP_GameInstance.BP_GameInstance_C|GetisHostDisqualified (Variables|Default|GetAs%20BP%20Game%20Instance%20Server)))
              (Variables|/Game/-Blueprints/-General/Core/BP_GameInstance.BP_GameInstance_C|SetisHostDisqualified (Variables|Default|GetAs%20BP%20Game%20Instance%20Server) true)
              (Utilities|Array|Add (Variables|Default|GetDisqualifiedPlayersIndexesToKick) _array_index_2 :!label _label_2))
            (else
              (goto _label_2)))
          (else
            (Variables|/Game/-Blueprints/-Gameplay/Core/BP_PS_Gameplay.BP_PS_Gameplay_C|SetPlayerState _asbp_ps_gameplay_2 "NewEnumerator1")
            (if (and (Variables|/Game/-Blueprints/-General/Core/BP_GameInstance.BP_GameInstance_C|GetisHostDisqualified (Variables|Default|GetAs%20BP%20Game%20Instance%20Server)) (Variables|/Game/-Blueprints/-Gameplay/Core/BP_PS_Gameplay.BP_PS_Gameplay_C|GetisHost _asbp_ps_gameplay_2))
              (Variables|/Game/-Blueprints/-Gameplay/Core/BP_PS_Gameplay.BP_PS_Gameplay_C|SetPlayerState _asbp_ps_gameplay_2 "NewEnumerator2"))))))))

(event Custom|StartShowNextLevelWidgetTimer
  (bind _returnvalue (Utilities|Time|SetTimerbyEvent (EventDispatchers|CreateEvent :!event Custom|UpdateTimeToShowNextLevelWidget) 1.0 true))
  (Variables|Default|SetShowNextLevelTimer _returnvalue))

(event Custom|UpdateTimeToShowNextLevelWidget
  (if (!= (Variables|Default|GetCountTimeToShowNextLevelWidget) 0)
    (bind _result (Math|Integer|DecrementInt (Variables|Default|GetCountTimeToShowNextLevelWidget))
      (:%20%20
        (if (== _result 0)
          (bind _returnvalue (Utilities|Time|SetTimerbyEvent (EventDispatchers|CreateEvent :!event Custom|UpdateTimeToStartNextLevel) 1.0 true))
          (Variables|Default|SetStartNextLevelTimer _returnvalue)
          (for _array_element (Variables|Default|GetPlayerArray)
            (bind _asbp_pc_gameplay (Utilities|Casting|CastToBP_PC_Gameplay (Components|GetOwner _array_element)))
            (bind _asbp_ps_gameplay (Utilities|Casting|CastToBP_PS_Gameplay _array_element))
            (if (and (Utilities|Enum|Equal(Enum) (Variables|/Game/-Blueprints/-Gameplay/Core/BP_PS_Gameplay.BP_PS_Gameplay_C|GetPlayerState _asbp_ps_gameplay) (Utilities|Enum|LiteralenumEnum_PlayerStates "NewEnumerator2")) (not (Pawn|IsLocalController _asbp_pc_gameplay)))
              (Default|GotoMenu _asbp_pc_gameplay)
              (else
                (Default|ShowNextLevelWidget _asbp_pc_gameplay)))))))))

(event Custom|UpdateTimeToStartNextLevel
  (if (!= (Variables|Default|GetCountTimeToStartNextLevel) 0)
    (bind _result (Math|Integer|DecrementInt (Variables|Default|GetCountTimeToStartNextLevel))
      (:%20%20
        (if (== _result 1)
          (for _array_element (Variables|Default|GetPlayerArray)
            (bind _asbp_pc_gameplay (Utilities|Casting|CastToBP_PC_Gameplay (Components|GetOwner _array_element)))
            (Default|ShowNextLevelWidgetWhiteScreen _asbp_pc_gameplay))
          (elif (== (Variables|Default|GetCountTimeToStartNextLevel) 0)
            (Default|ExecuteServerTravelConsoleCommand (Variables|Default|GetAs%20BP%20GM%20Gameplay%20Server))))))))

(event Custom|OnPlayerCountChanged
  (bind _playerarray (Variables|Default|GetPlayerArray))
  (bind _returnvalue (Utilities|Array|Length _playerarray))
  (bind (_map_name _min_players _max_players _type _win_condition _qualification_info_type _qualified_percent) (CallFunction|GetCurrentLevelInfoRowData))
  (switch Utilities|FlowControl|Switch|SwitchonEnum_LevelWinConditions _win_condition
    (:NewEnumerator0
      (Variables|Default|SetMaxQualificationInfoScore (Math|Float|Truncate (* _returnvalue (Math|Float|MakeLiteralFloat _qualified_percent)))))
    (:NewEnumerator1
      (Variables|Default|SetMaxQualificationInfoScore (- _returnvalue (Math|Float|Truncate (* _returnvalue (Math|Float|MakeLiteralFloat _qualified_percent))))))
    (:NewEnumerator2
      (if (Variables|/Game/-Blueprints/-General/Core/BP_GameInstance.BP_GameInstance_C|GetisHostDisqualified (Variables|Default|GetAs%20BP%20Game%20Instance%20Server))
        (Variables|Default|SetMaxQualificationInfoScore (- _returnvalue 2))
        (else
          (Variables|Default|SetMaxQualificationInfoScore (- _returnvalue 1)))))))

(event Custom|CallOnChatMessageSendToGameState
  (params (Sender :type String) (Message :type String) (MessageType :type Byte))
  (Default|CallOnChatMessageSendtoGameState Sender Message MessageType))

(event Custom|AddQualificationInfoScore
  (bind _result (Math|Integer|IncrementInt (Variables|Default|GetCurrentQualificationInfoScore))
    (:%20%20
      (Variables|Default|SetCurrentQualificationInfoScore _result)
      (CallFunction|CheckFinishRoundCondition))))

(event Custom|UpdateStartCountTime
  (if (!= (Variables|Default|GetCountTimeToStartGame) -1)
    (bind _result (Math|Integer|DecrementInt (Variables|Default|GetCountTimeToStartGame))
      (:%20%20
        (Variables|Default|SetCountTimeToStartGame _result)
        (CallFunction|CheckConditiontoStartGame)))))

(event Custom|CheckConditionToStartGame
  (if (== (Variables|Default|GetCountTimeToStartGame) 0)
    (Variables|Default|SetisGameStarted true)
    (for _array_element (Variables|Default|GetPlayerArray)
      (bind _asbp_pc_gameplay (Utilities|Casting|CastToBP_PC_Gameplay (Components|GetOwner _array_element))
        (:then
          (Default|EnablePlayerInput _asbp_pc_gameplay))
        (:CastFailed
          (CallFunction|PrintCastFailed self _asbp_pc_gameplay true true))))
    (elif (== (Variables|Default|GetCountTimeToStartGame) -1)
      (for _array_element_2 (Variables|Default|GetPlayerArray)
        (bind _asbp_pc_gameplay_2 (Utilities|Casting|CastToBP_PC_Gameplay (Components|GetOwner _array_element_2))
          (:then
            (Default|HideStartCountWidget _asbp_pc_gameplay_2))
          (:CastFailed
            (CallFunction|PrintCastFailed self _asbp_pc_gameplay_2 true true)))))))

(event Custom|Finish%20Round
  (CallFunction|DisqualifyPlayersLoosers)
  (bind _returnvalue (Utilities|Time|SetTimerbyEvent (EventDispatchers|CreateEvent :!event Custom|UpdateCountTimeToShowResultBoard) 1.0 true))
  (Variables|Default|SetShowResultsBoardTimer _returnvalue)
  (for _array_element (Variables|Default|GetPlayerArray)
    (bind _asbp_pc_gameplay (Utilities|Casting|CastToBP_PC_Gameplay (Components|GetOwner _array_element)))
    (Default|ShowRoundOverPopUpWidget _asbp_pc_gameplay)
    (Default|HideConstObjectiveGoalWidget _asbp_pc_gameplay)))

(event Custom|UpdateCountTimeToShowResultBoard
  (if (!= (Variables|Default|GetCountTimeToShowResultsBoard) 0)
    (bind _result (Math|Integer|DecrementInt (Variables|Default|GetCountTimeToShowResultsBoard))
      (:%20%20
        (if (== _result 0)
          (bind _type (CallFunction|GetCurrentLevelInfoRowData))
          (if (or (Utilities|Enum|Equal(Enum) _type (Utilities|Enum|LiteralenumEnum_LevelTypes "NewEnumerator2")) (== (- (Utilities|Array|Length (Variables|Default|GetPlayerArray)) (Utilities|Array|Length (Variables|Default|GetDisqualifiedPlayersIndexesToKick))) 1))
            (Default|ShowWinner (Variables|Default|GetBP%20Winner%20Board%20Server))
            (else
              (Default|ShowResultsBoard (Variables|Default|GetBP%20ResultsBoardServer)))))))))

(event Custom|Start%20Send%20All%20Players%20To%20Menu%20Timer
  (Utilities|Time|SetTimerbyEvent (delegate Custom|Send%20Players%20To%20Menu) 6e+01))

(event EventBeginPlay
  (if (Networking|IsServer)
    (bind _returnvalue (Utilities|Time|SetTimerbyEvent (EventDispatchers|CreateEvent :!event Custom|UpdateReadyCountTime) 1.0 true))
    (Variables|Default|SetPlayersReadyTimer _returnvalue)
    (bind _asbp_game_instance (Utilities|Casting|CastToBP_GameInstance (Game|GetGameInstance)))
    (Variables|Default|SetAs%20BP%20Game%20Instance%20Server _asbp_game_instance)
    (bind _asbp_gm_gameplay (Utilities|Casting|CastToBP_GM_Gameplay (Game|GetGameMode))
      (:then
        (bind _output_get (Variables|Default|SetAs%20BP%20GM%20Gameplay%20Server _asbp_gm_gameplay))
        (EventDispatchers|BindEventtoOnPlayerCountChanged _output_get (EventDispatchers|CreateEvent :!event Custom|OnPlayerCountChanged))
        (bind _returnvalue_2 (Actor|GetActorOfClass "/Game/-Blueprints/Actors/BP_ResultsBoard.BP_ResultsBoard_C"))
        (Variables|Default|SetBP%20ResultsBoardServer _returnvalue_2)
        (bind _returnvalue_3 (Actor|GetActorOfClass "/Game/-Blueprints/Actors/BP_WinnerBoard.BP_WinnerBoard_C"))
        (Variables|Default|SetBP%20Winner%20Board%20Server _returnvalue_3))
      (:CastFailed
        (CallFunction|PrintCastFailed self _asbp_gm_gameplay true true)))))

(event EventDestroyed
  (Utilities|Time|ClearandInvalidateTimerbyHandle (Variables|Default|GetPlayersReadyTimer))
  (Utilities|Time|ClearandInvalidateTimerbyHandle (Variables|Default|GetStartGameTimer))
  (Utilities|Time|ClearandInvalidateTimerbyHandle (Variables|Default|GetShowResultsBoardTimer))
  (Utilities|Time|ClearandInvalidateTimerbyHandle (Variables|Default|GetShowNextLevelTimer)))

(fn ConstructionScript)

(fn OnRepCurrentQualificationInfoScore
  (Default|CallOnPlayerQualificationInfoScoreAdded))

(fn OnRepCountTimetoStartGame
  (Default|CallOnGameStateCountTimetoStartGameUpdated))

(fn OnRepMaxQualificationInfoScore
  (Default|CallOnGameStatePlayerCountChanged))