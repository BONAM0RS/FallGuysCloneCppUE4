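; Game mode for the transition level that counts down, then has the server move the multiplayer session to gameplay.
; BeginPlay disables seamless travel, caches the game instance and starts a one-second looping timer that decrements CountTime.
; At zero, the server issues a ServerTravel console command with hardcoded L_DizzyHeights.
; An unused alternative opens the game instance's travel level as a listen server and tells each transition player controller to join.
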(event Custom|Init%20Game%20Instance
  (bind _asbp_game_instance (Utilities|Casting|CastToBP_GameInstance (Game|GetGameInstance)))
  (Variables|Default|SetAs%20BP%20Game%20Instance _asbp_game_instance))

(event Custom|ServerTravel
  (if (Networking|IsServer)
    (Development|ExecuteConsoleCommand (Utilities|String|Append "ServerTravel " "L_DizzyHeights") 0)
    (Development|PrintString "Travel to Gameplay" true true "(R=0.895833,G=0.535452,B=0.000000,A=1.000000)" 6e+01)))

(event Custom|UpdateTime
  (bind _result (Math|Integer|DecrementInt (Variables|Default|GetCountTime))
    (:%20%20
      (Variables|Default|SetCountTime _result)
      (if (== (Variables|Default|GetCountTime) 0)
        (CallFunction|ServerTravel)))))

(event Custom|ServerTravelByCustomLogic
  ;[1 1 1] My alternative way to travel levels in multiplayer, works in New editor window
  (if (Networking|IsServer)
    (Game|OpenLevel(byName) (Variables|/Game/-Blueprints/-General/Core/BP_GameInstance.BP_GameInstance_C|GetTravelLevelName (Variables|Default|GetAs%20BP%20Game%20Instance)) true "listen")
    (for _array_element (Variables|/Script/Engine.GameStateBase|GetPlayerArray (Game|GetGameState))
      (bind _asbp_pc_transition (Utilities|Casting|CastToBP_PC_Transition (Components|GetOwner _array_element)))
      (Default|SendJoinSessiontoClient _asbp_pc_transition))))

(event EventBeginPlay
  (bind _returnvalue (Utilities|Time|SetTimerbyEvent (delegate Custom|UpdateTime) 1.0 true))
  (Variables|Default|SetUpdateTimer _returnvalue)
  (Variables|Default|SetbUseSeamlessTravel false)
  (CallFunction|InitGameInstance))

(fn ConstructionScript)