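; BP_PC_Lobby is the lobby player controller, handling the return to the main menu and session travel for clients.
; The OpenMenu input opens L_Menu directly.
; SendJoinSessionToClient stores the travel level name in BP_GameInstance.
; On non-server instances it then destroys the current session and, on success, joins the game instance's saved JoinedSessionResult.
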(event Custom|SendJoinSessionToClient
  (params (TravelLevelName :type Name))
  (bind _asbp_game_instance (Utilities|Casting|CastToBP_GameInstance (Game|GetGameInstance)))
  (Variables|/Game/-Blueprints/-General/Core/BP_GameInstance.BP_GameInstance_C|SetTravelLevelName _asbp_game_instance TravelLevelName)
  (if (not (Networking|IsServer))
    (|DestroySession self
      (:OnSuccess
        (bind _asbp_game_instance_2 (Utilities|Casting|CastToBP_GameInstance (Game|GetGameInstance)))
        (Default|JoinSession _asbp_game_instance_2 self (Variables|/Game/-Blueprints/-General/Core/BP_GameInstance.BP_GameInstance_C|GetJoinedSessionResult _asbp_game_instance_2))))))

(event EventBeginPlay)

(event Input|ActionEvents|InputActionOpenMenu
  (params (Key :type Key%20Structure :default "None"))
  (:Pressed
    (Game|OpenLevel(byObjectReference) "/Game/-Maps/Menu/L_Menu.L_Menu")))

(fn ConstructionScript)