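; Lobby game mode that moves the multiplayer session from the lobby to a randomly chosen race level.
; BeginPlay caches the game instance, picks the level name and disables seamless travel to avoid carrying over actors and widgets.
; The travel event saves the connected player count to the game instance, then runs a ServerTravel console command.
; An older alternative opens the transition map as a listen server and has each lobby controller send a join to its client.
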(event Custom|ExecuteServerTravelConsoleCommand
  (bind _randomracelevelname (Variables|Default|GetRandomRaceLevelName))
  (bind _as_bp_game_instance (Variables|Default|GetAs%20BP%20Game%20Instance))
  (bind _returnvalue (Utilities|String|ToString(Name) _randomracelevelname))
  (Variables|/Game/-Blueprints/-General/Core/BP_GameInstance.BP_GameInstance_C|SetPlayersConnectedToLobby _as_bp_game_instance (Utilities|Array|Length (Variables|/Script/Engine.GameStateBase|GetPlayerArray (Game|GetGameState))))
  (Development|ExecuteConsoleCommand (Utilities|String|Append "ServerTravel " _returnvalue) 0)
  (Development|PrintString (Utilities|String|Append "Travel to " _returnvalue " hosted by " (Utilities|String|ToString(Text) (Variables|/Game/-Blueprints/-General/Core/BP_GameInstance.BP_GameInstance_C|GetPlayerName _as_bp_game_instance))) true true "(R=0.895833,G=0.535452,B=0.000000,A=1.000000)" 3.6e+02))

(event Custom|ServerTravelByCustomLogic
  ;[1 1 1] My alternative way to travel levels in multiplayer, works in New editor window (old code)
  (if (Networking|IsServer)
    (Game|OpenLevel(byObjectReference) "/Game/-Maps/Transition/L_Transition.L_Transition" true "listen")
    (for _array_element (Variables|/Script/Engine.GameStateBase|GetPlayerArray (Game|GetGameState))
      (bind _asbp_pc_lobby (Utilities|Casting|CastToBP_PC_Lobby (Components|GetOwner _array_element)))
      (Default|SendJoinSessiontoClient _asbp_pc_lobby "None"))))

(event EventBeginPlay
  (bind _asbp_game_instance (Utilities|Casting|CastToBP_GameInstance (Game|GetGameInstance))
    (:then
      (Variables|Default|SetAs%20BP%20Game%20Instance _asbp_game_instance)
      (bind _randomracelevelname (CallFunction|GetRandomGameplayRaceLevelName))
      (Variables|Default|SetRandomRaceLevelName _randomracelevelname)
      (Variables|Default|SetbUseSeamlessTravel false) ; Dont use seamless travel because it saves framework actors and then we need to clear them, widgets etc...
    )
    (:CastFailed
      (CallFunction|PrintCastFailed self _asbp_game_instance true true))))

(fn ConstructionScript)