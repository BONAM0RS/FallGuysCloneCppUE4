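; Lobby GameState that runs the pre-race countdown and triggers server travel when it ends or the lobby fills.
; On BeginPlay the server starts a looping one-second timer and reads the player cap from the level info of the GameMode's random race level.
; Each tick decrements CountTimeToStart and checks both start conditions before calling the GameMode's travel command.
; The countdown is RepNotify, broadcasting an update event on change.
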(event Custom|CheckConditionToStart
  (if (or (== (Variables|Default|GetCountTimeToStart) 0) (== (Utilities|Array|Length (Variables|Default|GetPlayerArray)) (Variables|Default|GetMaxPlayersToStart)))
    (Default|ExecuteServerTravelConsoleCommand (Variables|Default|GetAs%20BP%20GM%20Lobby))))

(event Custom|UpdateTime
  (if (!= (Variables|Default|GetCountTimeToStart) 0)
    (Variables|Default|SetCountTimeToStart (- (Variables|Default|GetCountTimeToStart) 1))
    (CallFunction|CheckConditiontoStart)))

(event EventBeginPlay
  (if (Networking|IsServer)
    (bind _returnvalue (Utilities|Time|SetTimerbyEvent (EventDispatchers|CreateEvent :!event Custom|UpdateTime) 1.0 true))
    (Variables|Default|SetUpdateTimer _returnvalue)
    (bind _asbp_gm_lobby (Utilities|Casting|CastToBP_GM_Lobby (Game|GetGameMode))
      (:then
        (Variables|Default|SetAs%20BP%20GM%20Lobby _asbp_gm_lobby)
        (bind _max_players (CallFunction|GetLevelInfoRowDatabyLevelName (Variables|/Game/-Blueprints/-Lobby/Core/BP_GM_Lobby.BP_GM_Lobby_C|GetRandomRaceLevelName (Variables|Default|GetAs%20BP%20GM%20Lobby))))
        (Variables|Default|SetMaxPlayersToStart _max_players))
      (:CastFailed
        (CallFunction|PrintCastFailed self _asbp_gm_lobby true true)))))

(event EventDestroyed
  (Utilities|Time|ClearandInvalidateTimerbyHandle (Variables|Default|GetUpdateTimer)))

(fn ConstructionScript)

(fn OnRepCountTimetoStart
  (Default|CallOnGameStateCountTimetoStartUpdated))